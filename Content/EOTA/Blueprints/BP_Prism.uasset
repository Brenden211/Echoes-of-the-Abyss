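; Rotatable light-puzzle prism that, while receiving light, emits a particle beam and relays it to the prism it hits.
; A forward line trace finds "Prism"-tagged actors and levels the beam endpoint to its own height.
; Activation spawns the beam after a delay, then messages and activates the hit prism, forming a chain.
; Interacting inside the trigger sphere deactivates the target, rotates a fixed step, re-traces and prunes old beams.
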(event OnComponentBeginOverlap(Triggersphere)
  (params (OverlappedComponent :type Primitive%20Component%20Object%20Reference) (OtherActor :type Actor%20Object%20Reference) (OtherComp :type Primitive%20Component%20Object%20Reference) (OtherBodyIndex :type Integer) (bFromSweep :type Boolean) (SweepResult :type Hit%20Result%20Structure%20%28by%20ref%29))
  (Variables|Default|SetCanInteract true))

(event OnComponentEndOverlap(Triggersphere)
  (params (OverlappedComponent :type Primitive%20Component%20Object%20Reference) (OtherActor :type Actor%20Object%20Reference) (OtherComp :type Primitive%20Component%20Object%20Reference) (OtherBodyIndex :type Integer))
  (Variables|Default|SetCanInteract false))

(event Custom|Update%20Light%20Source
  (bind _light_point (Variables|Default|GetLight%20point))
  (bind _output_get (Variables|Default|SetSelf%20Location (Transformation|GetWorldLocation _light_point)))
  (Variables|Default|SetEnd%20Location (+ _output_get (* (Math|Vector|GetForwardVector _light_point) (Variables|Default|GetEnd%20Location%20Length))))
  (CallFunction|LineforTarget))

(event Custom|Destroy%20Particle
  (CallFunction|UpdateLightSource)
  (if (> (Utilities|Array|Length (Variables|Default|GetLight%20Particle%20List)) 1)
    (Components|DestroyComponent (Utilities|Array|Get(acopy) (Variables|Default|GetLight%20Particle%20List)))
    (Utilities|Array|RemoveIndex (Variables|Default|GetLight%20Particle%20List))))

(event Custom|Line%20For%20Target
  (bind _outhit (Collision|LineTraceByChannel (Variables|Default|GetSelf%20Location) (Variables|Default|GetEnd%20Location) "TraceTypeQuery1" false 0 "None" true "(R=1.000000,G=0.000000,B=0.000000,A=1.000000)" "(R=0.000000,G=1.000000,B=0.000000,A=1.000000)" 1e+01))
  (bind _output_get (Variables|Default|SetOut%20Hit%20Actor (.hitactor _outhit)))
  (Utilities|IsValid _output_get
    (:Is%20Valid
      (if (Actor|ActorHasTag (.hitactor _outhit) "Prism")
        (bind _output_get_2 (Variables|Default|SetEnd%20Hit%20Location (Transformation|GetActorLocation (Variables|Default|GetOut%20Hit%20Actor))))
        (Variables|Default|SetEnd%20Location (+ (* (Variables|Default|GetSelf%20Location) "0.000000,0.000000,1.000000") (* _output_get_2 "1.000000,1.000000,0.000000")))
        (CallFunction|Activate)
        (else
          (Development|PrintString (Utilities|GetDisplayName (Variables|Default|GetOut%20Hit%20Actor))))))
    (:Is%20Not%20Valid
      (Development|PrintString "NO HIT")
      (Rendering|Debug|DrawDebugLine (Variables|Default|GetSelf%20Location) (Variables|Default|GetEnd%20Location) "(R=0.900354,G=0.270759,B=1.000000,A=1.000000)" 5.0 3.0)
      (CallFunction|Activate))))

(event EventBeginPlay
  (bind _light_point (Variables|Default|GetLight%20point))
  (bind _output_get (Variables|Default|SetSelf%20Location (Transformation|GetWorldLocation _light_point)))
  (Variables|Default|SetEnd%20Location (+ _output_get (* (Math|Vector|GetForwardVector _light_point) (Variables|Default|GetEnd%20Location%20Length))))
  (CallFunction|LineforTarget))

(event EventInteracted
  (if (Variables|Default|GetCanInteract)
    (Class|BPIPrism|DeactivateLight(Message) (Variables|Default|GetOut%20Hit%20Actor))
    (bind _output_get (Variables|Default|SetSelf%20Rotation (Transformation|GetWorldRotation (Variables|Default|GetDefaultSceneRoot))))
    (Transformation|SetWorldRotation (Variables|Default|GetDefaultSceneRoot) (Math|Rotator|CombineRotators _output_get "0.000000,35.000000,0.000000") false false)
    (CallFunction|DestroyParticle)))

(event EventActivate
  (if (Variables|Default|GetIsReceiving)
    (Utilities|FlowControl|Delay 1.0)
    (bind _returnvalue (Effects|SpawnEmitterAttached "/Game/EOTA/Niagara/CP_LightBeam_Prism.CP_LightBeam_Prism" (Variables|Default|GetLight%20point) "None" (Variables|Default|GetSelf%20Location) "0, 0, 0" "1.000000,1.000000,1.000000" "KeepWorldPosition" false))
    (bind _output_get (Variables|Default|SetLight%20Particle _returnvalue))
    (Utilities|IsValid _output_get
      (:Is%20Valid
        (Utilities|Array|Add (Variables|Default|GetLight%20Particle%20List) _output_get)
        (Class|ParticleSystemComponent|SetBeamSourcePoint (Variables|Default|GetLight%20Particle) 0 (Variables|Default|GetSelf%20Location))
        (Class|ParticleSystemComponent|SetBeamEndPoint (Variables|Default|GetLight%20Particle) 0 (Variables|Default|GetEnd%20Location))
        (Class|BPIPrism|ReceivingLight(Message) (Variables|Default|GetOut%20Hit%20Actor))
        (bind _asbp_prism (Utilities|Casting|CastToBP_Prism (Variables|Default|GetOut%20Hit%20Actor)))
        (Variables|BP_Prism_C|SetIsReceiving _asbp_prism true)
        (Class|BPIPrism|Activate(Message) (Variables|Default|GetOut%20Hit%20Actor))))))

(fn ConstructionScript)