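; BP_Doorway_Light is a doorway that opens and closes with the state of a linked light trigger.
; On BeginPlay it binds to the Trigger's IsLightActive event, if a valid Trigger is set.
; The ToggleDoor event hides the Cube and disables its collision while active, then shows it and restores query and physics collision when inactive.
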(event Custom|Toggle%20Door
  (params (IsActive :type Boolean))
  ;[0.3787 0.6401 1 1 30] Toggle the door
  (if IsActive
    (Collision|SetCollisionEnabled (Variables|Default|GetCube) "NoCollision")
    (Development|SetHiddeninGame (Variables|Default|GetCube) true false)
    (else
      (Collision|SetCollisionEnabled (Variables|Default|GetCube) "QueryAndPhysics")
      (Development|SetHiddeninGame (Variables|Default|GetCube) false false))))

(event EventBeginPlay
  (bind _trigger (Variables|Default|GetTrigger))
  (Utilities|IsValid _trigger
    (:Is%20Valid
      (EventDispatchers|BindEventtoIsLightActive _trigger (EventDispatchers|CreateEvent :!event Custom|Toggle%20Door)))))

(fn ConstructionScript)