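; Health component that shows a world-space health bar on its owning actor and tracks that actor's health.
; BeginPlay caches the WB_HealthBar widget and the BP_Paladin_FP player, whose camera the bar turns to face every tick.
; UpdateHealth converts incoming hits to damage with a flat minimum, updates the progress bar, and calls the owner's DeathMessage once health drops below zero.
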(event Custom|Update%20Health
  (params (In%20Hits :type Float%20%28double-precision%29))
  (bind _output_get (Variables|Default|SetDamage (+ (/ In%20Hits 1e+02) 0.1)))
  (Development|PrintString (Utilities|String|ToString(Float) _output_get))
  (bind _output_get_2 (Variables|Default|SetCurrent%20Health (- (Variables|Default|GetCurrent%20Health) (Variables|Default|GetDamage))))
  (if (> _output_get_2 -0.01)
    (CallFunction|SetHealthBar (Variables|Default|GetCurrent%20Health))
    (else
      (bind _output_get_3 (Variables|Default|SetCurrent%20Health -0.1))
      (CallFunction|SetHealthBar _output_get_3)
      (Class|BPIDamage|Death(Message) (Components|GetOwner)))))

(event Custom|Print%20Current%20Health
  (Development|PrintString (Utilities|String|ToString(Float) (Variables|/Script/UMG.ProgressBar|GetPercent (Variables|/Game/EOTA/UI/WB_HealthBar.WB_HealthBar_C|GetPGB_Healthbar (Variables|Default|GetAs%20WB%20Health%20Bar))))))

(event Custom|Look%20at%20Player
  (if (Variables|Default|GetPlayerValid)
    (bind _out_player_look_rotation (CallFunction|GetPlayerLookRotation))
    (Variables|Default|SetHealthBarRotation _out_player_look_rotation)
    (else
      (Variables|Default|SetHealthBarRotation (Transformation|GetWorldRotation self))))
  (Transformation|SetWorldRotation (Variables|Default|GetWBC%20Scene%20Component) (Variables|Default|GetHealthBarRotation) false false))

(event EventBeginPlay
  (bind _returnvalue (Components|GetOwner))
  (bind _returnvalue_2 (Actor|GetComponentbyClass _returnvalue "WBC_Health_C"))
  (bind _healthbar_widget_ (Variables|Default|GetHealthbar%20Widget%20)
    (:then
      (bind _returnvalue_3 (UserInterface|CreateWidget _healthbar_widget_))
      (Variables|Default|SetHealthbar%20Widget _returnvalue_3)
      (Utilities|IsValid _returnvalue_2
        (:Is%20Valid
          (Variables|Default|SetWBC%20Scene%20Component _returnvalue_2)
          (bind _asbp_paladin_fp (Utilities|Casting|CastToBP_Paladin_FP (Game|GetPlayerCharacter 0)))
          (Utilities|IsValid _asbp_paladin_fp
            (:Is%20Valid
              (Variables|Default|SetAs%20BP%20Knight%20FP _asbp_paladin_fp)
              (bind _aswb_health_bar (Utilities|Casting|CastToWB_HealthBar (UserInterface|GetWidget (Variables|Default|GetWBC%20Scene%20Component))))
              (Variables|Default|SetAs%20WB%20Health%20Bar _aswb_health_bar))))))
    (:else)))

(event EventTick
  (params (DeltaSeconds :type Float%20%28single-precision%29))
  (Utilities|IsValid (Variables|Default|GetAs%20BP%20Knight%20FP)
    (:Is%20Valid
      (Variables|Default|SetPlayerValid true))
    (:Is%20Not%20Valid
      (Variables|Default|SetPlayerValid false)))
  (CallFunction|LookatPlayer))

(fn SetHealthBar
  (params (In%20Health :type Float%20%28double-precision%29))
  (Progress|SetPercent (Variables|/Game/EOTA/UI/WB_HealthBar.WB_HealthBar_C|GetPGB_Healthbar (Variables|Default|GetAs%20WB%20Health%20Bar)) In%20Health))

(fn GetPlayerLookRotation
  (return (Math|Rotator|FindLookatRotation (Transformation|GetWorldLocation (Variables|Default|GetWBC%20Scene%20Component)) (Transformation|GetWorldLocation (Variables|/Game/EOTA/Blueprints/Character/Knight/BP_Paladin_FP.BP_Paladin_FP_C|GetFP%20Camera (Variables|Default|GetAs%20BP%20Knight%20FP))))))