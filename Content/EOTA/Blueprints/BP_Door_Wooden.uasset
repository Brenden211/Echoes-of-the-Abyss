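; BP_Door_Wooden is a wooden door that opens and closes when a linked lever is toggled.
; On BeginPlay it stores the door's world rotation and, if a Trigger is valid, binds to its OnLeverToggle event.
; ToggleDoor sets IsOpen from the lever state and snaps the door to a fixed absolute world rotation or back to the stored one, with no interpolation.
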(event Custom|Toggle%20Door
  (params (Lever%20Active :type Boolean))
  ;[1 0.9459 0 1 30] Toggle the door to open or close depending on the lever boolean
  (if Lever%20Active
    (Variables|Default|SetIsOpen true)
    (Transformation|SetWorldRotation (Variables|Default|GetDoor) "0.000000,75.000000,0.000000" false false)
    (else
      (Variables|Default|SetIsOpen false)
      (Transformation|SetWorldRotation (Variables|Default|GetDoor) (Variables|Default|GetOriginal%20Rotation) false false))))

(event EventBeginPlay
  (bind _trigger (Variables|Default|GetTrigger))
  (Variables|Default|SetOriginal%20Rotation (Transformation|GetWorldRotation (Variables|Default|GetDoor)))
  (Utilities|IsValid _trigger
    (:Is%20Valid
      (EventDispatchers|BindEventtoOnLeverToggle _trigger (EventDispatchers|CreateEvent :!event Custom|Toggle%20Door)))))

(fn ConstructionScript)

(fn BPDoorWoodenAutoGenFunc
  (params (Lever%20Active :type Boolean)))