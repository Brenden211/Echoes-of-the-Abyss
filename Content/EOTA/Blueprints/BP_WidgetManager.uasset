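; BP_WidgetManager creates and controls the loading screen and HUD widgets.
; On BeginPlay it applies the GameInstance's widget type, showing the loading screen with UI-only input or removing it.
; Only if a wooden chest exists, it binds widget-type, dungeon-generated and chest-radius dispatchers, then creates the HUD.
; Events can fast-finish loading or toggle HUD text, but the chest overlap handler is an empty branch.
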(event Custom|On%20Chest%20Overlap
  (params (ShowHUD :type Boolean))
  (if ShowHUD
    _))

(event Custom|Show%20Loading%20Widget
  (bind _returnvalue (Game|GetPlayerController 0))
  (bind _returnvalue_2 (UserInterface|CreateWidget "/Game/EOTA/UI/WB_LoadingScreen.WB_LoadingScreen_C" _returnvalue))
  (bind _output_get (Variables|References|SetLoadingScreen%20REF _returnvalue_2))
  (UserInterface|Viewport|AddtoViewport _output_get 0)
  (Variables|/Script/Engine.PlayerController|SetbShowMouseCursor _returnvalue true)
  (Input|SetInputModeUIOnly _returnvalue 0 "DoNotLock" false))

(event Custom|Create%20Widgets
  (bind _returnvalue (UserInterface|CreateWidget "/Game/EOTA/UI/WB_HUD.WB_HUD_C" (Game|GetPlayerController 0)))
  (bind _output_get (Variables|References|SetHUD%20REF _returnvalue))
  (UserInterface|Viewport|AddtoViewport _output_get 0))

(event Custom|Hide%20Loading%20Screen
  (Widget|RemovefromParent (Variables|References|GetLoadingScreen%20REF)))

(event Custom|Manage%20Widget%20Type
  (params (Enum%20Widget%20Type :type Enum_WidgetType%20Enum :default "NewEnumerator0"))
  (switch Utilities|FlowControl|Switch|SwitchonEnum_WidgetType Enum%20Widget%20Type
    (:NewEnumerator0
      (CallFunction|ShowLoadingWidget))
    (:NewEnumerator1
      (CallFunction|HideLoadingScreen))))

(event Custom|Finish%20Loading
  (Default|FastLoading (Variables|References|GetLoadingScreen%20REF)))

(event Custom|Manage%20Dispatchers
  (EventDispatchers|BindEventtoOnWidgetType (Variables|Casting|GetAs%20BP%20Main%20Game%20Instance) (EventDispatchers|CreateEvent :!event Custom|Manage%20Widget%20Type))
  (EventDispatchers|BindEventtoOnDungeonGenerated (Variables|Casting|GetAs%20BP%20Main%20Game%20Instance) (EventDispatchers|CreateEvent :!event Custom|Finish%20Loading))
  (EventDispatchers|BindEventtoOnChestRadiusOverlap (Variables|Casting|GetAS%20BP%20Chest%20Wooden) (EventDispatchers|CreateEvent :!event Custom|On%20Chest%20Overlap)))

(event EventBeginPlay
  (bind _asbp_main_game_instance (Utilities|Casting|CastToBP_MainGameInstance (Game|GetGameInstance)))
  (bind _output_get (Variables|Casting|SetAs%20BP%20Main%20Game%20Instance _asbp_main_game_instance))
  (CallFunction|ManageWidgetType (Variables|/Game/EOTA/Blueprints/BP_MainGameInstance.BP_MainGameInstance_C|GetEnumWidgetType _output_get))
  (bind _returnvalue (Actor|GetActorOfClass "/Game/EOTA/Blueprints/Actor/BP_Chest_Wooden.BP_Chest_Wooden_C"))
  (Utilities|IsValid _returnvalue
    (:Is%20Valid
      (Variables|Casting|SetAS%20BP%20Chest%20Wooden _returnvalue)
      (CallFunction|ManageDispatchers)
      (CallFunction|CreateWidgets))))

(event EventHideHUD
  (Widget|SetVisibility (Variables|References|GetHUD%20REF) "Hidden"))

(event EventShowHUD
  (params (In%20Message :type Text))
  (Default|SetText (Variables|References|GetHUD%20REF) In%20Message)
  (Widget|SetVisibility (Variables|References|GetHUD%20REF) "Visible"))

(fn ConstructionScript)