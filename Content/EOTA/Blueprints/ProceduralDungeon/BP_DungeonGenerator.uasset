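; Actor that procedurally builds a dungeon at BeginPlay by chaining random rooms from a start room onto random open exit points.
; After a short delay, each room's overlap boxes are checked; overlapping rooms are destroyed and retried, while valid ones add their exits to the pool.
; Once the room count is met, unused exits get walls.
; A looping timer opens the test map if generation exceeds a time limit.
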(event Custom|Spawn%20Start%20Room
  ;[0.3787 0.6401 1 1 30] Spawn start room
  (bind _returnvalue (Game|SpawnActorfromClass "/Game/EOTA/Blueprints/ProceduralDungeon/Rooms/BP_StartRoom.BP_StartRoom_C" (Transformation|GetWorldTransform (Variables|Default|GetDefaultSceneRoot)) "AlwaysSpawn" "MultiplyWithRoot" 0 0))
  (Utilities|Array|AppendArray (Variables|Default|GetExit%20List) (Components|GetChildrenComponents (Variables|/Game/EOTA/Blueprints/ProceduralDungeon/Rooms/BP_MasterRoom.BP_MasterRoom_C|GetExit%20Folder _returnvalue) false))
  (CallFunction|SpawnNextRoom))

(event Custom|Spawn%20Next%20Room
  ;[0.3787 0.6401 1 1 30] Spawns the next room and will keep spawning rooms while the max room amount is greater than 0.
  (Variables|Default|SetSelected%20Exit%20Point (.OutItem (Utilities|Array|Random (Variables|Default|GetExit%20List))))
  (bind _returnvalue (Game|SpawnActorfromClass (.OutItem (Utilities|Array|Random (Variables|Default|GetRoom%20List))) (Transformation|GetWorldTransform (Variables|Default|GetSelected%20Exit%20Point)) "AlwaysSpawn" "MultiplyWithRoot" 0 0))
  (bind _asbp_master_room (Utilities|Casting|CastToBP_MasterRoom _returnvalue))
  (Variables|Default|SetLatest%20Room _asbp_master_room)
  (Utilities|FlowControl|Delay (Variables|Default|GetTime%20Between%20Rooms))
  (CallFunction|CheckforOverlap))

(event Custom|Add%20Overlapping%20Rooms%20to%20List
  ;[0.3787 0.6401 1 1 30] Add overlapping rooms to list
  (for _array_element (Components|GetChildrenComponents (Variables|/Game/EOTA/Blueprints/ProceduralDungeon/Rooms/BP_MasterRoom.BP_MasterRoom_C|GetOverlap%20Folder (Variables|Default|GetLatest%20Room)) false)
    (bind _asbox_collision (Utilities|Casting|CastToBoxComponent _array_element))
    (Utilities|Array|AppendArray (Variables|Default|GetOverlaped%20List) (Class|PrimitiveComponent|GetOverlappingComponents _asbox_collision))))

(event Custom|Check%20for%20Overlap
  ;[0.3787 0.6401 1 1 30] Delete latest room if overlapping and keep spawning rooms. Also checks if all the rooms are spawned.
  (CallFunction|AddOverlappingRoomstoList)
  (if (Utilities|Array|IsNotEmpty (Variables|Default|GetOverlaped%20List))
    (Utilities|Array|Clear (Variables|Default|GetOverlaped%20List))
    (Actor|DestroyActor (Variables|Default|GetLatest%20Room))
    (CallFunction|SpawnNextRoom)
    (else
      (Utilities|Array|Clear (Variables|Default|GetOverlaped%20List))
      (Variables|Default|SetRoom%20Total (- (Variables|Default|GetRoom%20Total) 1))
      (Utilities|Array|RemoveItem (Variables|Default|GetExit%20List) (Variables|Default|GetSelected%20Exit%20Point))
      (Utilities|Array|AppendArray (Variables|Default|GetExit%20List) (Components|GetChildrenComponents (Variables|/Game/EOTA/Blueprints/ProceduralDungeon/Rooms/BP_MasterRoom.BP_MasterRoom_C|GetExit%20Folder (Variables|Default|GetLatest%20Room)) false))
      (if (> (Variables|Default|GetRoom%20Total) 0)
        (CallFunction|SpawnNextRoom)
        (else
          (Utilities|FlowControl|Delay (Variables|Default|GetClose%20Exits%20Delay))
          (CallFunction|CloseOpenedExits)
          (Variables|Default|SetDungeonComplete true)
          (Utilities|Time|ClearandInvalidateTimerbyHandle (Variables|Default|GetTimer%20Handle))
          (Development|PrintString "DUNGEON COMPLETE" true true "(R=1.000000,G=0.945882,B=0.000000,A=1.000000)" 5.0)
          (CallFunction|PrintDungeonRooms))))))

(event Custom|Close%20Opened%20Exits
  ;[0.3787 0.6401 1 1 30] Close all the exits that are not connected to any room.
  (for _array_element (Variables|Default|GetExit%20List)
    (Game|SpawnActorfromClass "/Game/EOTA/Blueprints/ProceduralDungeon/BP_DungeonExitWall.BP_DungeonExitWall_C" (Transformation|GetWorldTransform _array_element) "AlwaysSpawn" "MultiplyWithRoot" 0 0)))

(event Custom|Start%20Dungeon%20Timer
  ;[0.3787 0.6401 1 1 30] Dungeon Timer
  (bind _returnvalue (Utilities|Time|SetTimerbyEvent (delegate Custom|Check%20for%20Dungeon%20Complete) 0.5 true))
  (Variables|Default|SetTimer%20Handle _returnvalue))

(event Custom|Check%20for%20Dungeon%20Complete
  ;[0.3787 0.6401 1 1 30] Dungeon Timer
  (Development|PrintString "Running Timer")
  (if (>= (Utilities|Time|GetGameTimeinSeconds) (Variables|Default|GetMax%20Dungeon%20Time))
    (Game|OpenLevel(byName) "Map_ProceduralGenerationTest")))

(event EventBeginPlay
  (Variables|Default|SetRooms%20Spawned (Variables|Default|GetRoom%20Total))
  (CallFunction|SpawnStartRoom)
  (CallFunction|StartDungeonTimer))

(fn ConstructionScript)

(fn PrintDungeonRooms
  (Development|PrintString (Utilities|String|Append "ROOMS GENERATED: " (Utilities|String|ToString(Integer) (Variables|Default|GetRooms%20Spawned))) true true "(R=0.493814,G=0.348958,B=1.000000,A=1.000000)" 5.0))