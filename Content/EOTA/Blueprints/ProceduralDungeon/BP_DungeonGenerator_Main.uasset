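; Main procedural dungeon generator that builds the dungeon's fixed core and launches per-zone generator actors from its central hub.
; On BeginPlay it chains start room, hallway and hub at exit transforms, placing door frames on every collected exit.
; Each SpawnZone call matches a hub exit by display name, spawns that zone's generator if enabled, then advances ZoneIndex.
; BeginPlay triggers only one zone step; CloseExit, which walls listed exits after a delay, is uncalled here.
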(event Custom|Spawn%20Start%20Room
  ;[0.3787 0.6401 1 1 30] Spawn start room
  (bind _returnvalue (Game|SpawnActorfromClass "/Game/EOTA/Blueprints/ProceduralDungeon/DungeonRooms/Starting/BP_Dungeon_StartRoom.BP_Dungeon_StartRoom_C" (Transformation|GetWorldTransform (Variables|Components|GetDefaultSceneRoot)) "AlwaysSpawn" "MultiplyWithRoot" 0 0))
  (bind _output_get (Variables|Components|SetLatest%20Exit (Components|GetChildComponent (Variables|/Game/EOTA/Blueprints/ProceduralDungeon/DungeonRooms/BP_Dungeon_MasterRoom.BP_Dungeon_MasterRoom_C|GetExit%20Folder _returnvalue) 0)))
  (Utilities|Array|Add (Variables|ComponentList|GetExit%20List) _output_get)
  (CallFunction|SpawnStartHallway))

(event Custom|Spawn%20Start%20Hallway
  ;[0.3787 0.6401 1 1 30] Spawn start hallway after the starting room
  (bind _returnvalue (Game|SpawnActorfromClass "/Game/EOTA/Blueprints/ProceduralDungeon/DungeonRooms/Starting/BP_Dungeon_StartHallway.BP_Dungeon_StartHallway_C" (Transformation|GetWorldTransform (Variables|Components|GetLatest%20Exit)) "AlwaysSpawn" "MultiplyWithRoot" 0 0))
  (bind _output_get (Variables|Components|SetLatest%20Exit (Components|GetChildComponent (Variables|/Game/EOTA/Blueprints/ProceduralDungeon/DungeonRooms/BP_Dungeon_MasterRoom.BP_Dungeon_MasterRoom_C|GetExit%20Folder _returnvalue) 0)))
  (Utilities|Array|Add (Variables|ComponentList|GetExit%20List) _output_get)
  (CallFunction|SpawnCentralHub))

(event Custom|Spawn%20Zone%204
  ;[0.3787 0.6401 1 1 30] Spawns the zone 4
  (if (Variables|Zone4|GetbZone4)
    (Game|SpawnActorfromClass "/Game/EOTA/Blueprints/ProceduralDungeon/BP_DungeonGenerator_Zone4.BP_DungeonGenerator_Zone4_C" (Transformation|GetWorldTransform (Variables|Components|GetZone%20Exit)) "AlwaysSpawn" "MultiplyWithRoot" 0 (Variables|Zone4|GetZone4%20Room) "Zone 4" (Variables|Zone4|GetbChallengeRoom4) 0)))

(event Custom|Spawn%20Zone%201
  ;[0.3787 0.6401 1 1 30] Spawns the zone 1
  (if (Variables|Zone1|GetbZone1)
    (Game|SpawnActorfromClass "/Game/EOTA/Blueprints/ProceduralDungeon/BP_DungeonGenerator_Zone1.BP_DungeonGenerator_Zone1_C" (Transformation|GetWorldTransform (Variables|Components|GetZone%20Exit)) "AlwaysSpawn" "MultiplyWithRoot" 0 (Variables|Zone1|GetZone1%20Room) "ZONE 1" (Variables|Zone1|GetbChallengeRoom1) 0)))

(event Custom|Spawn%20Door%20Frame
  ;[0.3787 0.6401 1 1 30] Spawn the door frame at each exit
  (for _array_element (Variables|ComponentList|GetExit%20List)
    (Game|SpawnActorfromClass "/Game/EOTA/Blueprints/BP_DoorFrame.BP_DoorFrame_C" (Transformation|GetWorldTransform _array_element) "AlwaysSpawn" "MultiplyWithRoot" 0 0)))

(event Custom|Spawn%20Central%20Hub
  ;[0.3787 0.6401 1 1 30] Spawn central hub after the starting hallway room and set the central hub exits
  (bind _returnvalue (Game|SpawnActorfromClass "/Game/EOTA/Blueprints/ProceduralDungeon/DungeonRooms/Starting/BP_Dungeon_CentralHub.BP_Dungeon_CentralHub_C" (Transformation|GetWorldTransform (Variables|Components|GetLatest%20Exit)) "AlwaysSpawn" "MultiplyWithRoot" 0 0))
  (Utilities|Array|AppendArray (Variables|ComponentList|GetExit%20List) (Components|GetChildrenComponents (Variables|/Game/EOTA/Blueprints/ProceduralDungeon/DungeonRooms/BP_Dungeon_MasterRoom.BP_Dungeon_MasterRoom_C|GetExit%20Folder _returnvalue) false))
  (Variables|ComponentList|SetCentralHubExits (Components|GetChildrenComponents (Variables|/Game/EOTA/Blueprints/ProceduralDungeon/DungeonRooms/BP_Dungeon_MasterRoom.BP_Dungeon_MasterRoom_C|GetExit%20Folder _returnvalue) false))
  (CallFunction|SpawnDoorFrame))

(event Custom|Spawn%20Zone
  ;[0.3787 0.6401 1 1 30] Spawns the correct zone actor bp into the scene
  (switch int (Variables|Default|GetZone%20Index)
    (:0
      (CallFunction|SetZoneExit (Variables|ComponentList|GetCentralHubExits) (Variables|String|GetZone1%20Actor%20Name))
      (CallFunction|SpawnZone1))
    (:1
      (CallFunction|SetZoneExit (Variables|ComponentList|GetCentralHubExits) (Variables|String|GetZone2%20Actor%20Name))
      (CallFunction|SpawnZone2)
      (Development|PrintString "----------" true true "(R=0.000000,G=0.660000,B=1.000000,A=1.000000)" 15.0))
    (:2
      (CallFunction|SetZoneExit (Variables|ComponentList|GetCentralHubExits) (Variables|String|GetZone3%20Actor%20Name))
      (CallFunction|SpawnZone3)
      (Development|PrintString "----------" true true "(R=0.000000,G=0.660000,B=1.000000,A=1.000000)" 15.0))
    (:3
      (CallFunction|SetZoneExit (Variables|ComponentList|GetCentralHubExits) (Variables|String|GetZone4%20Actor%20Name))
      (CallFunction|SpawnZone4)
      (Development|PrintString "----------" true true "(R=0.000000,G=0.660000,B=1.000000,A=1.000000)" 15.0)))
  (Math|Integer|IncrementInt (Variables|Default|GetZone%20Index)))

(event Custom|Close%20Exit
  ;[1 1 1 0.5 30] Close all exits that are not connected to any room.
  (Utilities|FlowControl|Delay (Variables|Time|GetDelay%20Close%20Exit))
  (for _array_element (Variables|ComponentList|GetExit%20List)
    (Game|SpawnActorfromClass "/Game/EOTA/Blueprints/ProceduralDungeon/DungeonRooms/BP_Dungeon_Exit_Wall.BP_Dungeon_Exit_Wall_C" (Transformation|GetWorldTransform _array_element) "AlwaysSpawn" "MultiplyWithRoot" 0 0)))

(event Custom|Spawn%20Zone%202
  ;[0.3787 0.6401 1 1 30] Spawns the zone 2
  (if (Variables|Zone2|GetbZone2)
    (Game|SpawnActorfromClass "/Game/EOTA/Blueprints/ProceduralDungeon/BP_DungeonGenerator_Zone2.BP_DungeonGenerator_Zone2_C" (Transformation|GetWorldTransform (Variables|Components|GetZone%20Exit)) "AlwaysSpawn" "MultiplyWithRoot" 0 (Variables|Zone2|GetZone2%20Room) "Zone 2" (Variables|Zone2|GetbChallengeRoom2) 0)))

(event Custom|Spawn%20Zone%203
  ;[0.3787 0.6401 1 1 30] Spawns the zone 3
  (if (Variables|Zone3|GetbZone3)
    (Game|SpawnActorfromClass "/Game/EOTA/Blueprints/ProceduralDungeon/BP_DungeonGenerator_Zone3.BP_DungeonGenerator_Zone3_C" (Transformation|GetWorldTransform (Variables|Components|GetZone%20Exit)) "AlwaysSpawn" "MultiplyWithRoot" 0 (Variables|Zone3|GetZone3%20Room) "Zone 3" (Variables|Zone3|GetbChallengeRoom3) 0)))

(event EventBeginPlay
  (CallFunction|SpawnStartRoom)
  (CallFunction|SpawnZone))

(fn ConstructionScript)

(fn SetZoneExit
  (params (Exits :type Array%20of%20Scene%20Component%20Object%20References) (Zone%20Name :type String))
  (for _array_element Exits
    (LocalVariables|SetExit _array_element)
    (if (Utilities|Enum|Equal(Enum) (Utilities|GetDisplayName _array_element) Zone%20Name)
      (Variables|Components|SetZone%20Exit (LocalVariables|GetExit)))))