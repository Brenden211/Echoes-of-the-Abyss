(event Custom|Delete%20Dungeon
  ;[0.3787 0.6401 1 1 30] Delete the dungeon if failure to generate
  (for _array_element (Variables|Components|GetGenerated%20List)
    (Actor|DestroyActor _array_element))
  (CallFunction|ResetDungeon))

(event Custom|Spawn%20Random%20Room
  (bind _exit_list (Variables|Components|GetExit%20List))
  (bind _outitem (Utilities|Array|Random _exit_list))
  ;[0.3787 0.6401 1 1 30] Spawn a random room from the appropriate list
  (Utilities|FlowControl|Delay (Variables|Time|GetTime%20Between%20Rooms))
  (Utilities|IsValid _outitem
    (:Is%20Valid
      (bind _output_get (Variables|Components|SetSelected%20Exit%20Point _outitem))
      (bind _returnvalue (Game|SpawnActorfromClass (.OutItem (Utilities|Array|Random (Variables|RoomLists|GetRoom%20List))) (Transformation|GetWorldTransform _output_get) "AlwaysSpawn" "MultiplyWithRoot" 0 0))
      (bind _asbp_dungeon_master_room (Utilities|Casting|CastToBP_Dungeon_MasterRoom _returnvalue))
      (bind _output_get_2 (Variables|Components|SetLatest%20Room _asbp_dungeon_master_room))
      (Utilities|Array|Add (Variables|Components|GetGenerated%20List) _output_get_2)
      (CallFunction|AddOverlapRooms))
    (:Is%20Not%20Valid
      (Development|PrintString "UMM THE EXIT LIST IS EMPTY"))))

(event Custom|Spawn%20Challenge%20Room
  ;[0.3787 0.6401 1 1 30] Spawn a random challenge room
  (Utilities|FlowControl|Delay (Variables|Time|GetTime%20Between%20Rooms))
  (Variables|ZoneDetails|SetbTryChallengeRoom true)
  (bind _output_get (Variables|Components|SetSelected%20Exit%20Point (.OutItem (Utilities|Array|Random (Variables|Components|GetExit%20List)))))
  (bind _returnvalue (Game|SpawnActorfromClass (.OutItem (Utilities|Array|Random (Variables|RoomLists|GetChallenge%20Room%20List))) (Transformation|GetWorldTransform _output_get) "AlwaysSpawn" "MultiplyWithRoot" 0 0))
  (bind _asbp_dungeon_master_room (Utilities|Casting|CastToBP_Dungeon_MasterRoom _returnvalue))
  (bind _output_get_2 (Variables|Components|SetLatest%20Room _asbp_dungeon_master_room))
  (Utilities|Array|Add (Variables|Components|GetGenerated%20List) _output_get_2)
  (CallFunction|AddOverlapRooms))

(event Custom|Set%20Room
  ;[0.9602 1 0.2552 1 30] Check if the room total matches the goal, else keep spawning rooms
  (bind _result (Math|Integer|DecrementInt (Variables|ZoneDetails|GetRoom%20Needed))
    (:%20%20
      (Utilities|Array|Add (Variables|Components|GetDoor%20List) (Variables|Components|GetSelected%20Exit%20Point))
      (if (> _result 0)
        (if (Variables|ZoneDetails|GetbHasChallengeRoom)
          (CallFunction|SpawnRandomRoom :!label _label)
          (else
            (bind _output_value (CallFunction|PickChallengeRoom))
            (if _output_value
              (CallFunction|SpawnChallengeRoom)
              (else
                (CallFunction|IncreaseChallengeRoomChance)
                (goto _label)))))
        (else
          (Utilities|Time|ClearandInvalidateTimerbyHandle (Variables|Timer|GetDungeon%20Timer%20Handle))
          (CallFunction|CloseOpenExits)
          (CallFunction|SpawnDoorFrames)
          (Development|PrintString "Zone Complete" true true "(R=0.960229,G=1.000000,B=0.255208,A=1.000000)")
          (CallFunction|ActivateNextZone))))))

(event Custom|Reset%20Dungeon
  ;[0.9602 1 0.2552 1 30] Reset the dungeon if failure to generate
  (Utilities|Array|Clear (Variables|Components|GetGenerated%20List))
  (Utilities|Array|Clear (Variables|Components|GetExit%20List))
  (Utilities|Array|Clear (Variables|Components|GetDoor%20List))
  (Variables|ZoneDetails|SetRoom%20Needed (Variables|ZoneDetails|GetRoom%20Goal))
  (Variables|ZoneDetails|SetbHasChallengeRoom false)
  (Variables|ZoneDetails|SetbHasStartingRoom false)
  (Variables|ZoneDetails|SetbTryStartingRoom false)
  (Variables|ZoneDetails|SetbTryChallengeRoom false)
  (Utilities|Array|Clear (Variables|Default|GetCH%20Room%20Chance))
  (bind _result (Math|Integer|IncrementInt (Variables|ZoneDetails|GetZone%20Reset%20Current))
    (:%20%20
      ;;[0.3787 0.6401 1] If the dungeon takes more than 3 times to generate reset the level.
      (if (> _result (Variables|ZoneDetails|GetZone%20Reset%20Limit))
        (Game|OpenLevel(byObjectReference) "/Game/EOTA/Maps/MAP_ProceduralGenerationTest.MAP_ProceduralGenerationTest")))))

(event Custom|Spawn%20Starting%20Room
  ;[0.3787 0.6401 1 1 30] Spawn the starting room
  (Utilities|FlowControl|Delay (Variables|Time|GetTime%20Between%20Rooms))
  (Variables|ZoneDetails|SetbTryStartingRoom true)
  (bind _output_get (Variables|Components|SetSelected%20Exit%20Point (.OutItem (Utilities|Array|Random (Variables|Components|GetExit%20List)))))
  (bind _returnvalue (Game|SpawnActorfromClass "/Game/EOTA/Blueprints/ProceduralDungeon/DungeonRooms/Starting/BP_Dungeon_StartHallway.BP_Dungeon_StartHallway_C" (Transformation|GetWorldTransform _output_get) "AlwaysSpawn" "MultiplyWithRoot" 0 0))
  (bind _output_get_2 (Variables|Components|SetLatest%20Room _returnvalue))
  (Utilities|Array|Add (Variables|Components|GetGenerated%20List) _output_get_2)
  (Utilities|FlowControl|Delay (Variables|Time|GetTime%20Between%20Rooms))
  (CallFunction|AddOverlapRooms))

(event Custom|Increase%20Challenge%20Room%20Chance
  (bind _ch_room_chance (Variables|Default|GetCH%20Room%20Chance))
  (bind _returnvalue (Utilities|Array|Length _ch_room_chance))
  ;[0.3787 0.6401 1 1 30] Increase the challenge room chance
  (if (>= _returnvalue 0)
    (Utilities|Array|RemoveIndex (Variables|Default|GetCH%20Room%20Chance) (- _returnvalue 1))))

(event Custom|Delete%20Room
  (bind _latest_room (Variables|Components|GetLatest%20Room))
  ;[0.3787 0.6401 1 1 30] Delete the latest room that was placed if it overlaps with another room
  (Utilities|Array|Clear (Variables|Components|GetOverlapping%20List))
  (Actor|DestroyActor _latest_room)
  (Utilities|Array|RemoveItem (Variables|Components|GetGenerated%20List) _latest_room))

(event Custom|Add%20Overlap%20Rooms
  ;[0.3787 0.6401 1 1 30] Add any rooms that overlap with the latest room to the overlapping list
  (for _array_element (Components|GetChildrenComponents (Variables|/Game/EOTA/Blueprints/ProceduralDungeon/DungeonRooms/BP_Dungeon_MasterRoom.BP_Dungeon_MasterRoom_C|GetOverlap%20Folder (Variables|Components|GetLatest%20Room)) false)
    (bind _asbox_collision (Utilities|Casting|CastToBoxComponent _array_element))
    (Utilities|Array|AppendArray (Variables|Components|GetOverlapping%20List) (Class|PrimitiveComponent|GetOverlappingComponents _asbox_collision)))
  (CallFunction|CheckOverlap))

(event Custom|Check%20Overlap
  ;[0.9602 1 0.2552 1 30] If the overlapping list contains a room, delete the room and spawn a random room. If there are no rooms inside the overlapping list, continue
  (if (Utilities|Array|IsNotEmpty (Variables|Components|GetOverlapping%20List))
    (Development|PrintString "Delete Room")
    (CallFunction|DeleteRoom)
    (CallFunction|SpawnRandomRoom)
    (else
      (bind _output_exit_list (CallFunction|GetAllExits))
      (Utilities|Array|AppendArray (Variables|Components|GetExit%20List) _output_exit_list)
      (Utilities|Array|RemoveItem (Variables|Components|GetExit%20List) (Variables|Components|GetSelected%20Exit%20Point))
      (if (Variables|ZoneDetails|GetbTryStartingRoom)
        (Variables|ZoneDetails|SetbHasStartingRoom true))
      (if (Variables|ZoneDetails|GetbTryChallengeRoom)
        (Variables|ZoneDetails|SetbHasChallengeRoom true))
      (CallFunction|SetRoom))))

(event Custom|Spawn%20Door%20Frames
  ;[0.3787 0.6401 1 1 30] Spawn a door frame at each exit that is connected to a room
  (for _array_element (Variables|Components|GetDoor%20List)
    (Game|SpawnActorfromClass (.OutItem (Utilities|Array|Random (Variables|RoomLists|GetDoor%20Actor%20List))) (Transformation|GetWorldTransform _array_element) "AlwaysSpawn" "MultiplyWithRoot" 0 0)))

(event Custom|Close%20Open%20Exits
  ;[0.3787 0.6401 1 1 30] Place exit walls at the exits not connected to any room
  (for _array_element (Variables|Components|GetExit%20List)
    (Game|SpawnActorfromClass "/Game/EOTA/Blueprints/ProceduralDungeon/DungeonRooms/BP_Dungeon_Exit_Wall.BP_Dungeon_Exit_Wall_C" (Transformation|GetWorldTransform _array_element) "AlwaysSpawn" "MultiplyWithRoot" 0 0)))

(event Custom|Start%20Dungeon%20Timer
  ;[0.9602 1 0.2552 1 30] Start the stopwatch clock to track how long it takes to create
  (bind _returnvalue (Utilities|Time|SetTimerbyEvent (delegate Custom|Dungeon%20Timer%20Tick) 1.0 true))
  (Variables|Timer|SetDungeon%20Timer%20Handle _returnvalue))

(event Custom|Dungeon%20Timer%20Tick
  ;[0.9602 1 0.2552 1 30] Start the stopwatch clock to track how long it takes to create
  (Development|PrintText (Utilities|Text|FormatText (Utilities|Text|ToText(Integer) (Variables|Timer|GetTimer%20Seconds))))
  (bind _result (Math|Integer|IncrementInt (Variables|Timer|GetTimer%20Seconds))
    (:%20%20
      (if (>= _result 10)
        (CallFunction|DeleteDungeon)
        (CallFunction|SetupDungeon)))))

(event Custom|Setup%20Dungeon
  ;[0.9602 1 0.2552 1 30] Set the values for the dungeon before starting the timer
  (bind _ouput_zone_exit (CallFunction|GetZoneExit))
  (Utilities|Array|Add (Variables|Components|GetExit%20List) _ouput_zone_exit)
  (Variables|ZoneDetails|SetRoom%20Needed (Variables|ZoneDetails|GetRoom%20Goal))
  (Variables|Timer|SetBuild%20Time%20Limit (/ (Variables|ZoneDetails|GetRoom%20Goal) 5))
  (CallFunction|SetChallengeRoomChance)
  (CallFunction|SpawnStartingRoom))

(event Custom|Activate%20Next%20Zone
  ;[0.3787 0.6401 1 1 30] Activate the next zone
  (Default|SpawnZone (Variables|Components|GetBP%20Dungeon%20Generator%20Main) (Variables|Timer|GetTimer%20Seconds)))

(event EventBeginPlay
  (Utilities|FlowControl|Delay 0.1)
  (CallFunction|StartDungeonTimer)
  (CallFunction|SetupDungeon))

(fn ConstructionScript)

(fn SetHasStartingRoom
  (Variables|ZoneDetails|SetbHasStartingRoom true)
  (Variables|ZoneDetails|SetbTryStartingRoom false))

(fn SetHasChallengeRoom
  (Variables|ZoneDetails|SetbHasChallengeRoom true)
  (Variables|ZoneDetails|SetbTryChallengeRoom false))

(fn SetChallengeRoomChance
  (bind _room_goal (Variables|ZoneDetails|GetRoom%20Goal))
  (bind _returnvalue (- _room_goal 2))
  (bind _output_get (LocalVariables|SetTemp%20Room%20Goal _returnvalue))
  (while (> _output_get 0)
    (if (== (LocalVariables|GetTemp%20Room%20Goal) _returnvalue)
      (Utilities|Array|Add (Variables|Default|GetCH%20Room%20Chance) 1)
      (else
        (Utilities|Array|Add (Variables|Default|GetCH%20Room%20Chance) 0)))
    (Math|Integer|DecrementInt (LocalVariables|GetTemp%20Room%20Goal))))

(fn GetAllExits
  (return (Components|GetChildrenComponents (Variables|/Game/EOTA/Blueprints/ProceduralDungeon/DungeonRooms/BP_Dungeon_MasterRoom.BP_Dungeon_MasterRoom_C|GetExit%20Folder (Variables|Components|GetLatest%20Room)) false)))

(fn GetZoneExit
  (bind _returnvalue (Actor|GetActorOfClass "/Game/EOTA/Blueprints/ProceduralDungeon/BP_DungeonGenerator_Starting.BP_DungeonGenerator_Starting_C"))
  (Utilities|IsValid _returnvalue
    (:Is%20Valid
      (bind _output_get (Variables|Components|SetBP%20Dungeon%20Generator%20Main _returnvalue))
      (return (Variables|/Game/EOTA/Blueprints/ProceduralDungeon/BP_DungeonGenerator_Starting.BP_DungeonGenerator_Starting_C|GetZone%20Exit _output_get)))
    (:Is%20Not%20Valid
      (Development|PrintString "NOT VALID CAST"))))

(fn PickChallengeRoom
  (return (== (.OutItem (Utilities|Array|Random (Variables|Default|GetCH%20Room%20Chance))) 1)))