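; Procedural generator for dungeon Zone 2, growing rooms from the main generator's ExitZone2 after a fixed hallway and Lucky layout.
; Spawns random rooms at random open exits, destroying and retrying any that overlap, until the room count is met.
; Then walls off unused exits and places stream-picked doors at connections.
; A looping timer restarts failed builds with a time limit extended by half.
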(event Custom|Reset%20Dungeon
  ;[1 1 1 0.5 30] Reset the dungeon if it fails to generate
  (Development|PrintString "DUNGEON FAILED" true true "(R=0.900354,G=0.270759,B=1.000000,A=1.000000)" 5.0)
  (for _array_element (Variables|Components|GetGenerated%20List)
    (Actor|DestroyActor _array_element))
  (Utilities|Time|ClearandInvalidateTimerbyHandle (Variables|Timer|GetTimer%20Handle))
  (Utilities|Array|Clear (Variables|Components|GetGenerated%20List))
  (Utilities|Array|Clear (Variables|Components|GetExit%20List))
  (Utilities|Array|Clear (Variables|Components|GetDoor%20List))
  (Variables|Integers|SetRoom%20Needed (Variables|Integers|GetRoom%20Total))
  (Variables|Time|SetDungeon%20Time%20Elasped 0)
  (CallFunction|SpawnFirstRoom)
  (CallFunction|StartDungeonTimer))

(event Custom|Spawn%20Random%20Room
  ;[0.3787 0.6401 1 1 30] Spawns a random room from a random exit
  (Variables|Components|SetSelected%20Exit%20Point (.OutItem (Utilities|Array|Random (Variables|Components|GetExit%20List))))
  (bind _returnvalue (Game|SpawnActorfromClass (.OutItem (Utilities|Array|Random (Variables|RoomLists|GetRoom%20List))) (Transformation|GetWorldTransform (Variables|Components|GetSelected%20Exit%20Point)) "AlwaysSpawn" "MultiplyWithRoot" 0 0))
  (bind _asbp_dungeon_master_room (Utilities|Casting|CastToBP_Dungeon_MasterRoom _returnvalue))
  (bind _output_get (Variables|Components|SetLatest%20Room _asbp_dungeon_master_room))
  (Utilities|Array|Add (Variables|Components|GetGenerated%20List) _output_get)
  (Utilities|FlowControl|Delay (Variables|Time|GetTime%20Between%20Rooms))
  (CallFunction|CheckforOverlap))

(event Custom|Add%20Overlapping%20Rooms%20to%20List
  ;[0.3787 0.6401 1 1 30] Add overlapping rooms to list
  (for _array_element (Components|GetChildrenComponents (Variables|/Game/EOTA/Blueprints/ProceduralDungeon/DungeonRooms/BP_Dungeon_MasterRoom.BP_Dungeon_MasterRoom_C|GetOverlap%20Folder (Variables|Components|GetLatest%20Room)) false)
    (bind _asbox_collision (Utilities|Casting|CastToBoxComponent _array_element))
    (Utilities|Array|AppendArray (Variables|Components|GetOverlaped%20List) (Class|PrimitiveComponent|GetOverlappingComponents _asbox_collision))))

(event Custom|Check%20for%20Overlap
  (bind _latest_room (Variables|Components|GetLatest%20Room))
  ;[0.3787 0.6401 1 1 30] Delete latest room if overlapping and keep spawning rooms. Also checks if all the rooms are spawned.
  (CallFunction|AddOverlappingRoomstoList)
  (if (Utilities|Array|IsNotEmpty (Variables|Components|GetOverlaped%20List))
    (Utilities|Array|Clear (Variables|Components|GetOverlaped%20List))
    (Actor|DestroyActor _latest_room)
    (Utilities|Array|RemoveItem (Variables|Components|GetGenerated%20List) _latest_room)
    (CallFunction|SpawnRandomRoom)
    (else
      (Utilities|Array|Clear (Variables|Components|GetOverlaped%20List))
      (Variables|Integers|SetRoom%20Needed (- (Variables|Integers|GetRoom%20Needed) 1))
      (Utilities|Array|RemoveItem (Variables|Components|GetExit%20List) (Variables|Components|GetSelected%20Exit%20Point))
      ;;[0.3787 0.6401 1] Add arrow to door list
      (Utilities|Array|Add (Variables|Components|GetDoor%20List) (Variables|Components|GetSelected%20Exit%20Point))
      (Utilities|Array|AppendArray (Variables|Components|GetExit%20List) (Components|GetChildrenComponents (Variables|/Game/EOTA/Blueprints/ProceduralDungeon/DungeonRooms/BP_Dungeon_MasterRoom.BP_Dungeon_MasterRoom_C|GetExit%20Folder (Variables|Components|GetLatest%20Room)) false))
      (if (> (Variables|Integers|GetRoom%20Needed) 0)
        (CallFunction|SpawnRandomRoom)
        (else
          (Utilities|FlowControl|Delay (Variables|Time|GetClose%20Exits%20Delay))
          (CallFunction|CloseOpenedExits)
          (CallFunction|SpawnDoors)
          (Utilities|Time|ClearandInvalidateTimerbyHandle (Variables|Timer|GetTimer%20Handle))
          (CallFunction|PrintTime)
          (CallFunction|PrintRooms)
          (Variables|Booleans|SetDungeonComplete true)
          (Actor|GetActorOfClass "/Game/EOTA/Blueprints/ProceduralDungeon/BP_DungeonGenerator_Main.BP_DungeonGenerator_Main_C"))))))

(event Custom|Spawn%20Doors
  ;[0.3787 0.6401 1 1 30] Spawn doors
  (for _array_element (Variables|Components|GetDoor%20List)
    (Game|SpawnActorfromClass (.OutItem (Utilities|Array|RandomFromStream (Variables|RoomLists|GetDoor%20Actor%20List) (Variables|Default|GetStream))) (Transformation|GetWorldTransform _array_element) "AlwaysSpawn" "MultiplyWithRoot" 0 0)))

(event Custom|Close%20Opened%20Exits
  ;[0.3787 0.6401 1 1 30] Close all the exits that are not connected to any room.
  (for _array_element (Variables|Components|GetExit%20List)
    (Game|SpawnActorfromClass "/Game/EOTA/Blueprints/ProceduralDungeon/DungeonRooms/BP_Dungeon_Exit_Wall.BP_Dungeon_Exit_Wall_C" (Transformation|GetWorldTransform _array_element) "AlwaysSpawn" "MultiplyWithRoot" 0 0)))

(event Custom|Start%20Dungeon%20Timer
  ;[0.3787 0.6401 1 1 30] Dungeon Timer
  (bind _returnvalue (Utilities|Time|SetTimerbyEvent (delegate Custom|Check%20for%20Dungeon%20Complete) 1.0 true))
  (Variables|Timer|SetTimer%20Handle _returnvalue))

(event Custom|Check%20for%20Dungeon%20Complete
  ;[0.3787 0.6401 1 1 30] Dungeon Timer
  (Development|PrintString "Timer Running")
  (if (>= (Utilities|Time|GetGameTimeinSeconds) (Variables|Timer|GetDungeon%20Build%20Time))
    (Variables|Booleans|SetDungeonFailed true)
    (Variables|Timer|SetDungeon%20Build%20Time (* (Variables|Timer|GetDungeon%20Build%20Time) 1.5))
    (CallFunction|ResetDungeon)))

(event Custom|Spawn%20First%20Room
  ;[0.3787 0.6401 1 1 30] Spawns the starting room from the zone1 exit from the actor BP class, then sets the latest room and adds the exits to the exit list
  (bind _returnvalue (Actor|GetActorOfClass "/Game/EOTA/Blueprints/ProceduralDungeon/BP_DungeonGenerator_Main.BP_DungeonGenerator_Main_C"))
  (bind _returnvalue_2 (Game|SpawnActorfromClass "/Game/EOTA/Blueprints/ProceduralDungeon/DungeonRooms/Zone1/BP_Dungeon_HallwayLong.BP_Dungeon_HallwayLong_C" (Transformation|GetWorldTransform (Variables|/Game/EOTA/Blueprints/ProceduralDungeon/BP_DungeonGenerator_Main.BP_DungeonGenerator_Main_C|GetExit%20Zone2 _returnvalue)) "AlwaysSpawn" "MultiplyWithRoot" 0 0))
  (bind _output_get (Variables|Components|SetLatest%20Room _returnvalue_2))
  (Utilities|Array|Add (Variables|Components|GetGenerated%20List) _output_get)
  (bind _returnvalue_3 (Game|SpawnActorfromClass "/Game/EOTA/Blueprints/ProceduralDungeon/DungeonRooms/Layout/BP_Dungeon_Layout_Lucky.BP_Dungeon_Layout_Lucky_C" (Transformation|GetWorldTransform (Variables|/Game/EOTA/Blueprints/ProceduralDungeon/DungeonRooms/Zone1/BP_Dungeon_HallwayLong.BP_Dungeon_HallwayLong_C|GetExit3 _returnvalue_2)) "AlwaysSpawn" "MultiplyWithRoot" 0 0))
  (bind _output_get_2 (Variables|Components|SetLatest%20Room _returnvalue_3))
  (Utilities|Array|Add (Variables|Components|GetGenerated%20List) _output_get_2)
  (Utilities|Array|AppendArray (Variables|Components|GetExit%20List) (Components|GetChildrenComponents (Variables|/Game/EOTA/Blueprints/ProceduralDungeon/DungeonRooms/BP_Dungeon_MasterRoom.BP_Dungeon_MasterRoom_C|GetExit%20Folder _output_get_2) false))
  (CallFunction|SpawnRandomRoom))

(event EventBeginPlay
  (Variables|Integers|SetRoom%20Total (Variables|Integers|GetRoom%20Needed))
  (CallFunction|SetDungeonBuildTime)
  (CallFunction|SpawnFirstRoom)
  (CallFunction|StartDungeonTimer))

(fn ConstructionScript)

(fn PrintRooms
  (Development|PrintString (Utilities|String|Append "ZONE 1 GENERATED: " (Utilities|String|ToString(Integer) (Variables|Integers|GetRoom%20Total))) true true "(R=0.493814,G=0.348958,B=1.000000,A=1.000000)" 5.0))

(fn PrintTime
  (Development|PrintString (Utilities|String|Append "DUNGEON COMPLETE: " (Utilities|String|ToString(Float) (Utilities|Time|GetGameTimeinSeconds))) true true "(R=1.000000,G=0.945882,B=0.000000,A=1.000000)" 5.0))

(fn RemoveFailedRoom
  (for _array_element (Variables|Components|GetGenerated%20List)
    (Actor|DestroyActor _array_element)))

(fn SetDungeonBuildTime
  (Variables|Timer|SetDungeon%20Build%20Time (/ (Math|Conversions|ToFloat(Integer) (Variables|Integers|GetRoom%20Needed)) 2.0)))