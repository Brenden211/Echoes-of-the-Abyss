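; BP_Dungeon_CH_Prism is a procedural dungeon challenge room with helpers for pairing levers with doors.
; Functions gather child actor components under door and lever folders into lists and pick random entries from them.
; Cast helpers toggle a BP_Doorway_Wood or assign a door to a BP_Lever.
; BeginPlay and construction only call the parent, and nothing here invokes the helpers.
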(event EventBeginPlay
  (|CallParentFunction))

(fn ConstructionScript
  (|CallParentFunction))

(fn SetDoorList
  (params (In%20Door%20Folder :type Scene%20Component%20Object%20Reference))
  (for _array_element (Components|GetChildrenComponents In%20Door%20Folder false)
    (bind _aschild_actor_component (Utilities|Casting|CastToChildActorComponent _array_element))
    (Utilities|Array|Add (LocalVariables|GetDoorList) _aschild_actor_component))
  (return (LocalVariables|GetDoorList)))

(fn CastToggleDoor
  (params (In%20Door :type Actor%20Object%20Reference))
  (bind _asbp_doorway_wood (Utilities|Casting|CastToBP_Doorway_Wood In%20Door))
  (Default|ToggleDoor _asbp_doorway_wood))

(fn SelectRandomDoor
  (params (In%20Door%20List :type Array%20of%20Child%20Actor%20Component%20Object%20References))
  (LocalVariables|SetDoorList In%20Door%20List)
  (if (> (Utilities|Array|Length (LocalVariables|GetDoorList)) 0)
    (return (Variables|/Script/Engine.ChildActorComponent|GetChildActor (.OutItem (Utilities|Array|Random (LocalVariables|GetDoorList)))) (.OutItem (Utilities|Array|Random (LocalVariables|GetDoorList))))))

(fn SetLeverList
  (params (In%20Lever%20Folder :type Scene%20Component%20Object%20Reference))
  (for _array_element (Components|GetChildrenComponents In%20Lever%20Folder false)
    (bind _aschild_actor_component (Utilities|Casting|CastToChildActorComponent _array_element))
    (Utilities|Array|Add (LocalVariables|GetLever%20List) _aschild_actor_component))
  (return (LocalVariables|GetLever%20List)))

(fn CastSetLevertoDoor
  (params (In%20Lever :type Actor%20Object%20Reference) (In%20Door :type Actor%20Object%20Reference))
  (bind _asbp_lever (Utilities|Casting|CastToBP_Lever In%20Lever))
  (Default|SetDoortoLever _asbp_lever In%20Door))

(fn SelectRandomLever
  (params (In%20Lever%20List :type Array%20of%20Child%20Actor%20Component%20Object%20References))
  (LocalVariables|SetLeverList In%20Lever%20List)
  (if (> (Utilities|Array|Length (LocalVariables|GetLeverList)) 0)
    (return (Variables|/Script/Engine.ChildActorComponent|GetChildActor (.OutItem (Utilities|Array|Random (LocalVariables|GetLeverList)))) (.OutItem (Utilities|Array|Random (LocalVariables|GetLeverList))))))