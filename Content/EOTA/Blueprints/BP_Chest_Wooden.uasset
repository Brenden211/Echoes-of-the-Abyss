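; BP_Chest_Wooden is a wooden chest that opens when interacted with.
; An IsOpen flag, cleared on BeginPlay, lets the Interacted event call Open only while the chest is closed, and nothing here closes it again.
; Open sets the flag and plays the OpenChest timeline, whose Rotation track is scaled to drive the pitch of the ChestCover's relative rotation.
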(event Custom|Open
  (Variables|Default|SetIsOpen true)
  (bind _rotation (Timeline|Open%20Chest Play)
    (:Update
      (Transformation|SetRelativeRotation (Variables|Default|GetChest%20Cover) (Math|Rotator|MakeRotator 0.0 (* _rotation 215.0) 0.0) false false))))

(event EventInteracted
  (if (not (Variables|Default|GetIsOpen))
    (CallFunction|Open)))

(event EventBeginPlay
  (Variables|Default|SetIsOpen false))

(fn ConstructionScript)