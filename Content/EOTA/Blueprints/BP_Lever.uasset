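; BP_Lever is an interactable lever that the knight player can toggle on and off while standing in range.
; InteractBox overlaps set CanInteract and, on each entry, bind to the knight's PlayerInteracted dispatcher, which is never unbound.
; LeverToggle checks CanInteract, flips IsActive, and snaps Handle between a fixed world rotation and the one saved at BeginPlay.
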(event OnComponentBeginOverlap(InteractBox)
  (params (OverlappedComponent :type Primitive%20Component%20Object%20Reference) (OtherActor :type Actor%20Object%20Reference) (OtherComp :type Primitive%20Component%20Object%20Reference) (OtherBodyIndex :type Integer) (bFromSweep :type Boolean) (SweepResult :type Hit%20Result%20Structure%20%28by%20ref%29))
  (bind _asbp_knight_fp (Utilities|Casting|CastToBP_Knight_FP OtherActor))
  (Variables|Default|SetCanInteract true)
  (EventDispatchers|BindEventtoPlayerInteracted _asbp_knight_fp (EventDispatchers|CreateEvent :!event Custom|Lever%20Toggle))
  (Development|PrintString "Inside"))

(event OnComponentEndOverlap(InteractBox)
  (params (OverlappedComponent :type Primitive%20Component%20Object%20Reference) (OtherActor :type Actor%20Object%20Reference) (OtherComp :type Primitive%20Component%20Object%20Reference) (OtherBodyIndex :type Integer))
  (Utilities|Casting|CastToBP_Knight_FP OtherActor)
  (Variables|Default|SetCanInteract false)
  (Development|PrintString "Outside"))

(event Custom|Lever%20Toggle
  (if (Variables|Default|GetCanInteract)
    (if (Variables|Default|GetIsActive)
      (Variables|Default|SetIsActive false)
      (Transformation|SetWorldRotation (Variables|Default|GetHandle) (Variables|Default|GetOriginalRotation) false false)
      (else
        (Variables|Default|SetIsActive true)
        (Transformation|SetWorldRotation (Variables|Default|GetHandle) "135.000000,0.000000,0.000000" false false)))))

(event EventBeginPlay
  (Variables|Default|SetOriginalRotation (Transformation|GetWorldRotation (Variables|Default|GetHandle))))

(fn ConstructionScript)