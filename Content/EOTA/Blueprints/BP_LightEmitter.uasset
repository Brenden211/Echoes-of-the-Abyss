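; BP_LightEmitter is a light source that fires a beam at a crystal in line with it, powering it.
; On BeginPlay it runs one visibility trace forward from its Cube, drawing a debug line if nothing is hit.
; An actor tagged "CH Light" is cast to BP_Crystal, set powered and sent ActivateMessage after the beam spawns.
; The yellow beam particle ends at the crystal's XY but keeps the emitter's height, staying horizontal.
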(event Custom|Line%20For%20Target
  (bind _outhit (Collision|LineTraceByChannel (Variables|Default|GetSelf%20Location) (Variables|Default|GetEnd%20Location) "TraceTypeQuery1" false 0 "None" true "(R=1.000000,G=0.000000,B=0.000000,A=1.000000)" "(R=0.000000,G=1.000000,B=0.000000,A=1.000000)" 1e+01))
  (bind _output_get (Variables|Default|SetOut%20Hit%20Actor (.hitactor _outhit)))
  (Utilities|IsValid _output_get
    (:Is%20Valid
      (if (Actor|ActorHasTag (.hitactor _outhit) "CH Light")
        (Variables|Default|SetEnd%20Hit%20Location (Transformation|GetActorLocation (Variables|Default|GetOut%20Hit%20Actor)))
        (Variables|Default|SetIsHit true)
        (bind _asbp_crystal (Utilities|Casting|CastToBP_Crystal (Variables|Default|GetOut%20Hit%20Actor)))
        (Variables|/Game/EOTA/Blueprints/BP_Crystal.BP_Crystal_C|SetIsPowered _asbp_crystal true)
        (CallFunction|ActivateBeam)
        (Class|BPIPrism|Activate(Message) (Variables|Default|GetOut%20Hit%20Actor))))
    (:Is%20Not%20Valid
      (Development|PrintString "NO HIT")
      (Rendering|Debug|DrawDebugLine (Variables|Default|GetSelf%20Location) (Variables|Default|GetEnd%20Location) "(R=0.900354,G=0.270759,B=1.000000,A=1.000000)" 5.0 3.0))))

(event Custom|Activate%20Beam
  (Utilities|FlowControl|Sequence
    (:then_0
      (bind _returnvalue (Effects|SpawnEmitterAttached "/Game/EOTA/Niagara/CP_LightBeam_Yellow.CP_LightBeam_Yellow" (Variables|Default|GetCube) "None" (Variables|Default|GetSelf%20Location) "0, 0, 0" "1.000000,1.000000,1.000000" "KeepWorldPosition"))
      (Variables|Default|SetLightParticle _returnvalue))
    (:then_1
      (if (Variables|Default|GetIsHit)
        (Class|ParticleSystemComponent|SetBeamSourcePoint (Variables|Default|GetLightParticle) 0 (Variables|Default|GetSelf%20Location))
        (Class|ParticleSystemComponent|SetBeamEndPoint (Variables|Default|GetLightParticle) 0 (+ (* (Variables|Default|GetSelf%20Location) "0.000000,0.000000,1.000000") (* (Variables|Default|GetEnd%20Hit%20Location) "1.000000,1.000000,0.000000")))))))

(event EventBeginPlay
  (bind _cube (Variables|Default|GetCube))
  (bind _output_get (Variables|Default|SetSelf%20Location (Transformation|GetWorldLocation _cube)))
  (Variables|Default|SetEnd%20Location (+ _output_get (* (Math|Vector|GetForwardVector _cube) 2e+03)))
  (CallFunction|LineforTarget))

(fn ConstructionScript)