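; Game instance that drives the main menu flow and relays dungeon and widget events through dispatchers.
; Shortly after init it shows WB_MainMenu with UI-only input if the startup level matches the target level.
; Start Game opens MAP_MainDungeon and removes the menu, with start and continue each broadcasting a widget type.
; A DungeonReady event sets a ready flag and broadcasts that generation is complete.
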(event Custom|Show%20Main%20Menu
  (bind _returnvalue (Game|GetPlayerController 0))
  (if (Utilities|Enum|Equal(Enum) (Variables|Default|GetCurrent%20Level) (Variables|Default|GetTarget%20Level))
    (Variables|Default|SetEnumWidgetType "NewEnumerator0")
    (bind _returnvalue_2 (UserInterface|CreateWidget "/Game/EOTA/UI/WB_MainMenu.WB_MainMenu_C" _returnvalue))
    (bind _output_get (Variables|Default|SetMainMenu%20REF _returnvalue_2))
    (UserInterface|Viewport|AddtoViewport _output_get 0)
    (Variables|/Script/Engine.PlayerController|SetbShowMouseCursor _returnvalue true)
    (Input|SetInputModeUIOnly _returnvalue 0 "DoNotLock" false)
    (EventDispatchers|AssignOnButtonClicked (Variables|Default|GetMainMenu%20REF) (EventDispatchers|CreateEvent :!event Custom|OnMenuButtonClicked))))

(event Custom|Dungeon%20Ready
  (Variables|Default|SetDungeonReady true)
  (Development|PrintString "Dungeon Completed" true true "(R=0.630208,G=0.000000,B=0.018121,A=1.000000)" 5.0)
  (Default|CallOnDungeonGenerated))

(event Custom|OnMenuButtonClicked
  (params (Button%20Type :type Enum_MenuButtonType%20Enum :default "NewEnumerator0"))
  (switch Utilities|FlowControl|Switch|SwitchonEnum_MenuButtonType Button%20Type
    (:NewEnumerator0
      (CallFunction|StartGame)
      (Widget|RemovefromParent (Variables|Default|GetMainMenu%20REF)))))

(event Custom|Continue%20Button%20Clicked
  (Default|CallOnWidgetType "NewEnumerator1"))

(event Custom|Start%20Game
  (Game|OpenLevel(byName) "MAP_MainDungeon")
  (Default|CallOnWidgetType "NewEnumerator0"))

(event EventInit
  (bind _returnvalue (Game|GetCurrentLevelName true))
  (Variables|Default|SetCurrent%20Level _returnvalue)
  (Utilities|FlowControl|Delay 0.1)
  (CallFunction|ShowMainMenu))