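; BP_Doorway is a door that other logic can open or close through its OpenDoor and CloseDoor events.
; At BeginPlay it stores the Door component's world rotation as the closed pose.
; Opening snaps the door to a hard-coded absolute world rotation rather than an offset from that pose, and closing restores the stored rotation.
; Both events update an IsOpen flag, with no interpolation or animation.
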(event Custom|Close%20Door
  ;[0.3787 0.6401 1 1 30] Close the door
  (Variables|Default|SetIsOpen false)
  (Transformation|SetWorldRotation (Variables|Default|GetDoor) (Variables|Default|GetOriginal%20Rotation) false false))

(event Custom|Open%20Door
  ;[0.3787 0.6401 1 1 30] Open the door
  (Variables|Default|SetIsOpen true)
  (Transformation|SetWorldRotation (Variables|Default|GetDoor) "0.000000,75.000000,0.000000" false false))

(event EventBeginPlay
  (Variables|Default|SetOriginal%20Rotation (Transformation|GetWorldRotation (Variables|Default|GetDoor))))

(fn ConstructionScript)