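; Light-relay crystal for a beam puzzle that, when powered, emits a particle beam and rotates in fixed steps on interaction.
; A forward line trace finds the hit actor; the beam snaps to tagged light objects or steps back short of other blockers.
; Hit actors receive interface messages, so crystals power and activate each other in chains and light receivers respond.
; Interaction deactivates the current target, destroys the old beam, then re-traces and re-activates.
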(event OnComponentBeginOverlap(Triggersphere)
  (params (OverlappedComponent :type Primitive%20Component%20Object%20Reference) (OtherActor :type Actor%20Object%20Reference) (OtherComp :type Primitive%20Component%20Object%20Reference) (OtherBodyIndex :type Integer) (bFromSweep :type Boolean) (SweepResult :type Hit%20Result%20Structure%20%28by%20ref%29))
  ;[1 1 1 0.5 30] When inside self collision trigger, set interact to true
  (Variables|Default|SetCanInteract true))

(event OnComponentEndOverlap(Triggersphere)
  (params (OverlappedComponent :type Primitive%20Component%20Object%20Reference) (OtherActor :type Actor%20Object%20Reference) (OtherComp :type Primitive%20Component%20Object%20Reference) (OtherBodyIndex :type Integer))
  ;[1 1 1 0.5 30] When outside self collision trigger, set interact to false
  (Variables|Default|SetCanInteract false))

(event Custom|Set%20Light%20Points
  ;[1 1 1 0.5 30] Set the particle start point and end point
  (Class|ParticleSystemComponent|SetBeamSourcePoint (Variables|Default|GetLight%20Particle) 0 (Variables|Default|GetSelf%20Location))
  (Class|ParticleSystemComponent|SetBeamEndPoint (Variables|Default|GetLight%20Particle) 0 (Variables|Default|GetEnd%20Location)))

(event Custom|Start%20Light%20Source
  (bind _light_point (Variables|Default|GetLight%20point))
  ;[1 1 1 0.5 30] Set self and end location to the default values
  (bind _output_get (Variables|Default|SetSelf%20Location (Transformation|GetWorldLocation _light_point)))
  (Variables|Default|SetEnd%20Location (+ _output_get (* (Math|Vector|GetForwardVector _light_point) 2e+03))))

(event Custom|Activate%20Hit%20Actor
  ;[1 1 1 0.5 30] Calls the interface events for the Light Reciever and the Crystal on the hit actor
  (Class|BPIPrism|ReceivingLight(Message) (Variables|Default|GetOut%20Hit%20Actor))
  (bind _asbp_crystal (Utilities|Casting|CastToBP_Crystal (Variables|Default|GetOut%20Hit%20Actor)))
  (Variables|BP_Crystal_C|SetIsPowered _asbp_crystal true)
  (Class|BPIPrism|Activate(Message) (Variables|Default|GetOut%20Hit%20Actor)))

(event Custom|Set%20End%20Hit%20Location
  ;[1 1 1 0.5 30] Set end hit location to the hit actor and set the end location to the hit actor position X, Y values and self Z value
  (bind _output_get (Variables|Default|SetEnd%20Hit%20Location (Transformation|GetActorLocation (Variables|Default|GetOut%20Hit%20Actor))))
  (Variables|Default|SetEnd%20Location (+ (* (Variables|Default|GetSelf%20Location) "0.000000,0.000000,1.000000") (* _output_get "1.000000,1.000000,0.000000"))))

(event Custom|Destroy%20Particle
  ;[1 1 1 0.5 30] Destroy the particle in the 0 index of the light particle list if the list has more than 1 particle
  (CallFunction|StartLightSource)
  (if (> (Utilities|Array|Length (Variables|Default|GetLight%20Particle%20List)) 0)
    (Components|DestroyComponent (Utilities|Array|Get(acopy) (Variables|Default|GetLight%20Particle%20List)))
    (Utilities|Array|RemoveIndex (Variables|Default|GetLight%20Particle%20List))))

(event Custom|Line%20For%20Target
  ;[1 1 1 0.5 30] Line trace to get the actor and if the tag matches, set the end hit location and end location but the end location only uses the z position of self location
  (bind _outhit (Collision|LineTraceByChannel (Variables|Default|GetSelf%20Location) (Variables|Default|GetEnd%20Location) "TraceTypeQuery1" false 0 "None" true "(R=1.000000,G=0.000000,B=0.000000,A=1.000000)" "(R=0.000000,G=1.000000,B=0.000000,A=1.000000)" 1e+01))
  (Rendering|Debug|DrawDebugLine (Variables|Default|GetSelf%20Location) (Variables|Default|GetEnd%20Location) "(R=0.900354,G=0.270759,B=1.000000,A=1.000000)" 1.0 3.0)
  (bind _output_get (Variables|Default|SetOut%20Hit%20Actor (.hitactor _outhit)))
  (Utilities|IsValid _output_get
    (:Is%20Valid
      (Variables|Default|SetisLightObj (Actor|ActorHasTag (.hitactor _outhit) "Light Obj"))
      (Variables|Default|SetIsLineHit true))
    (:Is%20Not%20Valid
      (Variables|Default|SetIsLineHit false))))

(event Custom|Find%20Before%20Location
  (bind _light_point (Variables|Default|GetLight%20point))
  ;[1 1 1 0.5 30] Find the location right before the hit actor and set end location to the new location
  (Variables|Default|SetEnd%20Location%20Length 2e+03)
  (while (Variables|Default|GetIs%20Trace%20Hit)
    (bind _output_get (Variables|Default|SetEnd%20Location (+ (Transformation|GetWorldLocation _light_point) (* (Math|Vector|GetForwardVector _light_point) (Variables|Default|GetEnd%20Location%20Length)))))
    (bind _outhit (Collision|LineTraceByChannel (Variables|Default|GetSelf%20Location) _output_get "TraceTypeQuery1" false 0 "None" true "(R=1.000000,G=0.000000,B=0.000000,A=1.000000)" "(R=0.000000,G=1.000000,B=0.000000,A=1.000000)" 1e+01))
    (bind _output_get_2 (Variables|Default|SetOut%20Hit%20Actor (.hitactor _outhit)))
    (Utilities|IsValid _output_get_2
      (:Is%20Valid
        (Variables|Default|SetIs%20Trace%20Hit true)
        (Variables|Default|SetEnd%20Location%20Length (- (Variables|Default|GetEnd%20Location%20Length) 5.0)))
      (:Is%20Not%20Valid
        (Variables|Default|SetIs%20Trace%20Hit false))))
  (Variables|Default|SetIs%20Trace%20Hit true))

(event EventBeginPlay
  (bind _light_point (Variables|Default|GetLight%20point))
  (bind _output_get (Variables|Default|SetSelf%20Location (Transformation|GetWorldLocation _light_point)))
  (Variables|Default|SetEnd%20Location (+ _output_get (* (Math|Vector|GetForwardVector _light_point) 2e+03)))
  (CallFunction|LineforTarget))

(event EventInteracted
  ;[1 1 1 0.5 30] Interface event from Knight_FP when interacted will deactivate the light from the hit actor and rotate the crystal 35 degrees
  (if true
    (Class|BPIPrism|DeactivateLight(Message) (Variables|Default|GetOut%20Hit%20Actor))
    (bind _output_get (Variables|Default|SetSelf%20Rotation (Transformation|GetWorldRotation (Variables|Default|GetDefaultSceneRoot))))
    (Transformation|SetWorldRotation (Variables|Default|GetDefaultSceneRoot) (Math|Rotator|CombineRotators _output_get "0.000000,45.000000,0.000000") false false)
    (CallFunction|DestroyParticle)
    (CallFunction|LineforTarget)
    (CallFunction|Activate)))

(event EventActivate
  ;[1 1 1 0.5 30] Interface event from Light Emitter will spawn the particle emitter at self location and adds the particle to the light particle list
  (if (Variables|Default|GetIsPowered)
    (Utilities|FlowControl|Delay 1.0)
    (bind _returnvalue (Effects|SpawnEmitterAttached "/Game/EOTA/Niagara/CP_LightBeam_Crystal.CP_LightBeam_Crystal" (Variables|Default|GetLight%20point) "None" (Variables|Default|GetSelf%20Location) "0, 0, 0" "1.000000,1.000000,1.000000" "KeepWorldPosition" false))
    (bind _output_get (Variables|Default|SetLight%20Particle _returnvalue))
    (Utilities|IsValid _output_get
      (:Is%20Valid
        (Utilities|Array|Add (Variables|Default|GetLight%20Particle%20List) _output_get)
        (if (Variables|Default|GetIsLineHit)
          (if (Variables|Default|GetisLightObj)
            (CallFunction|SetEndHitLocation)
            (else
              (CallFunction|FindBeforeLocation)))
          (CallFunction|SetLightPoints)
          (CallFunction|ActivateHitActor)
          (else
            (CallFunction|SetLightPoints)))))
    (else
      (Development|PrintString "No Power"))))

(fn ConstructionScript)