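; BP_AltarRelic is an altar that displays a zone relic for the player to pick up.
; On BeginPlay it maps its relic enum to a class in LootRelics and spawns it at ItemSpawnPoint.
; Overlapping InteractCollision shows a widget-manager prompt if the player holds no relic.
; The Interacted event destroys the displayed relic, opens the relic UI and records the held type in BP_MainGameInstance, enforcing one relic at a time.
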(event OnComponentBeginOverlap(InteractCollision)
  (params (OverlappedComponent :type Primitive%20Component%20Object%20Reference) (OtherActor :type Actor%20Object%20Reference) (OtherComp :type Primitive%20Component%20Object%20Reference) (OtherBodyIndex :type Integer) (bFromSweep :type Boolean) (SweepResult :type Hit%20Result%20Structure%20%28by%20ref%29))
  (bind _output_get (Variables|Default|SetOverlap%20Actor OtherActor))
  (bind _holding_relic (CallFunction|GetNotHoldingRelic))
  (Variables|Default|SetIsOverlap true)
  (if (Math|Boolean|ANDBoolean _holding_relic (Actor|ActorHasTag _output_get "Player") (Variables|Default|GetCanInteract) (Variables|Default|GetAltarHasLoot))
    (Class|BPIHUD|ShowInteractUI(Message) (Variables|Default|GetAS%20BP%20Widget%20Manager) (Variables|Default|GetHUD%20Message))))

(event OnComponentEndOverlap(InteractCollision)
  (params (OverlappedComponent :type Primitive%20Component%20Object%20Reference) (OtherActor :type Actor%20Object%20Reference) (OtherComp :type Primitive%20Component%20Object%20Reference) (OtherBodyIndex :type Integer))
  (bind _output_get (Variables|Default|SetOverlap%20Actor OtherActor))
  (Variables|Default|SetIsOverlap false)
  (if (and (Actor|ActorHasTag _output_get "Player") (Variables|Default|GetCanInteract))
    (Class|BPIHUD|HideInteractUI(Message) (Variables|Default|GetAS%20BP%20Widget%20Manager))))

(event Custom|Event%20Spawn%20Relic
  (CallFunction|SpawnRelic (Variables|Default|GetEnum%20Relic%20Loot))
  (Variables|Default|SetAltarHasLoot true))

(event EventBeginPlay
  (bind _asbp_main_game_instance (Utilities|Casting|CastToBP_MainGameInstance (Game|GetGameInstance)))
  (Variables|Default|SetAs%20BP%20Main%20Game%20Instance _asbp_main_game_instance)
  (bind _returnvalue (Actor|GetActorOfClass "/Game/EOTA/Blueprints/BP_WidgetManager.BP_WidgetManager_C"))
  (Variables|Default|SetAS%20BP%20Widget%20Manager _returnvalue)
  (CallFunction|EventSpawnRelic))

(event EventInteracted
  (bind _holding_relic (CallFunction|GetNotHoldingRelic))
  (if (Math|Boolean|ANDBoolean _holding_relic (Variables|Default|GetAltarHasLoot) (Variables|Default|GetCanInteract) (Variables|Default|GetIsOverlap))
    (Actor|DestroyActor (Variables|Default|GetSpawnActorREF))
    (Variables|Default|SetAltarHasLoot false)
    (Default|ToggleRelicUI (Variables|Default|GetAS%20BP%20Widget%20Manager) true)
    (Default|SetRelicType (Variables|Default|GetAs%20BP%20Main%20Game%20Instance) (Variables|Default|GetEnum%20Relic%20Loot) true)))

(event EventHideInteractUI
  ;[0.3787 0.6401 1 0.6 30] Hide the interact UI
  (Class|BPIHUD|HideInteractUI(Message) (Variables|Default|GetAS%20BP%20Widget%20Manager)))

(fn ConstructionScript)

(fn SpawnRelic
  (params (Enum%20Relic :type Enum_RelicType%20Enum :default "NewEnumerator6"))
  (bind _item_spawn_point (Variables|Default|GetItem%20spawn%20point))
  (switch Utilities|FlowControl|Switch|SwitchonEnum_RelicType Enum%20Relic
    (:NewEnumerator6
      (Variables|Default|SetIndexRelicType 0))
    (:NewEnumerator0
      (Variables|Default|SetIndexRelicType 1))
    (:NewEnumerator1
      (Variables|Default|SetIndexRelicType 2))
    (:NewEnumerator2
      (Variables|Default|SetIndexRelicType 3))
    (:NewEnumerator5
      (Variables|Default|SetIndexRelicType 4)))
  (bind _returnvalue (Game|SpawnActorfromClass (Utilities|Array|Get(acopy) (Variables|Default|GetLootRelics) (Variables|Default|GetIndexRelicType)) (Math|Transform|MakeTransform (Transformation|GetWorldLocation _item_spawn_point) (Transformation|GetWorldRotation _item_spawn_point) "1.000000,1.000000,1.000000") "AlwaysSpawn" "MultiplyWithRoot" 0 0))
  (Variables|Default|SetSpawnActorREF _returnvalue))

(fn GetNotHoldingRelic
  (return (not (Variables|/Game/EOTA/Blueprints/BP_MainGameInstance.BP_MainGameInstance_C|GetHoldingRelic (Variables|Default|GetAs%20BP%20Main%20Game%20Instance)))))