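; BP_RelicZ1 is a relic actor that shows a HUD message while the first-person knight is within its interaction radius.
; BeginPlay caches the BP_Knight_FP and BP_WidgetManager instances through GetActorOfClass lookups.
; InteractRadius begin and end overlaps record the overlapping actor and overlap flag for any actor, but only tell the widget manager to show or hide the message for the knight.
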(event OnComponentBeginOverlap(InteractRadius)
  (params (OverlappedComponent :type Primitive%20Component%20Object%20Reference) (OtherActor :type Actor%20Object%20Reference) (OtherComp :type Primitive%20Component%20Object%20Reference) (OtherBodyIndex :type Integer) (bFromSweep :type Boolean) (SweepResult :type Hit%20Result%20Structure%20%28by%20ref%29))
  (bind _output_get (Variables|Default|SetOverlap%20Actor OtherActor))
  (Variables|Default|SetIsOverlap true)
  (if (== _output_get (Variables|Default|GetTarget%20Actor))
    (Class|BPIHUD|ShowHUD(Message) (Variables|Default|GetAS%20BP%20Widget%20Manager) (Variables|Default|GetHUD%20Message))))

(event OnComponentEndOverlap(InteractRadius)
  (params (OverlappedComponent :type Primitive%20Component%20Object%20Reference) (OtherActor :type Actor%20Object%20Reference) (OtherComp :type Primitive%20Component%20Object%20Reference) (OtherBodyIndex :type Integer))
  (bind _output_get (Variables|Default|SetOverlap%20Actor OtherActor))
  (Variables|Default|SetIsOverlap false)
  (if (== _output_get (Variables|Default|GetTarget%20Actor))
    (Class|BPIHUD|HideHUD(Message) (Variables|Default|GetAS%20BP%20Widget%20Manager))))

(event EventBeginPlay
  (bind _returnvalue (Actor|GetActorOfClass "/Game/EOTA/Blueprints/Character/Knight/BP_Knight_FP.BP_Knight_FP_C"))
  (Variables|Default|SetTarget%20Actor _returnvalue)
  (bind _returnvalue_2 (Actor|GetActorOfClass "/Game/EOTA/Blueprints/BP_WidgetManager.BP_WidgetManager_C"))
  (Variables|Default|SetAS%20BP%20Widget%20Manager _returnvalue_2))

(fn ConstructionScript)