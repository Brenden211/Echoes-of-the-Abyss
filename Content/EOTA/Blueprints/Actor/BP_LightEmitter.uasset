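; Puzzle-style light emitter actor that, when interacted with, fires a yellow beam at a "Light Obj" ahead and activates it.
; An overlap trigger enables interaction and shows a HUD prompt to the player through BP_WidgetManager while unpowered.
; Interacting line-traces forward from the particle spawn point, fits the beam particle's end to the hit distance, then messages the target.
; Power is set once the beam spawns, blocking further interaction.
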(event OnComponentBeginOverlap(Interact)
  (params (OverlappedComponent :type Primitive%20Component%20Object%20Reference) (OtherActor :type Actor%20Object%20Reference) (OtherComp :type Primitive%20Component%20Object%20Reference) (OtherBodyIndex :type Integer) (bFromSweep :type Boolean) (SweepResult :type Hit%20Result%20Structure%20%28by%20ref%29))
  ;[0.3787 0.6401 1 0.6 30] When inside self collision trigger, set interact to true
  (bind _output_get (Variables|Default|SetOverlap%20Actor OtherActor))
  (Variables|Default|SetCanInteract true)
  (if (and (Actor|ActorHasTag _output_get "Player") (and (Variables|Default|GetCanInteract) (not (Variables|Default|GetbPower))))
    (Class|BPIHUD|ShowInteractUI(Message) (Variables|Default|GetAS%20BP%20Widget%20Manager) (Variables|Default|GetHUD%20Message))))

(event OnComponentEndOverlap(Interact)
  (params (OverlappedComponent :type Primitive%20Component%20Object%20Reference) (OtherActor :type Actor%20Object%20Reference) (OtherComp :type Primitive%20Component%20Object%20Reference) (OtherBodyIndex :type Integer))
  ;[0.3787 0.6401 1 0.6 30] When outside self collision trigger, set interact to false
  (bind _output_get (Variables|Default|SetOverlap%20Actor OtherActor))
  (Variables|Default|SetCanInteract false)
  (if (Actor|ActorHasTag _output_get "Player")
    (Class|BPIHUD|HideInteractUI(Message) (Variables|Default|GetAS%20BP%20Widget%20Manager))))

(event Custom|Test%20For%20Target
  ;[0.3787 0.6401 1 0.6 30] Line trace to find an object in front, if object matches then setup light beam locations and spawn particle
  (bind _outhit (Collision|LineTraceByChannel (Variables|Default|GetSelf%20Location) (Variables|Default|GetEnd%20Location) "TraceTypeQuery1" false 0 "ForDuration" true "(R=1.000000,G=0.000000,B=0.000000,A=1.000000)" "(R=0.000000,G=1.000000,B=0.000000,A=1.000000)" 1.0))
  (Variables|Default|SetOut%20Hit%20Distance (+ (.distance _outhit) 15.0))
  (bind _output_get (Variables|Default|SetOut%20Hit%20Actor (.hitactor _outhit)))
  (Utilities|IsValid _output_get
    (:Is%20Valid
      (Variables|Default|SetbLineHit true)
      (if (Actor|ActorHasTag _output_get "Light Obj")
        (Variables|Default|SetbLineMatch true)
        (CallFunction|SetActorLocation)
        (CallFunction|SpawnLightBeam)
        (CallFunction|ActivateHitActor)))
    (:Is%20Not%20Valid
      (Variables|Default|SetbLineHit false))))

(event Custom|Spawn%20Lightbeam
  ;[0.3787 0.6401 1 0.6 30] Spawn the particle at self location and set the start and end location of the effect to the hit actor location
  (bind _returnvalue (Effects|SpawnEmitterAttached "/Game/EOTA/Niagara/CP_LightBeam_Yellow.CP_LightBeam_Yellow" (Variables|Default|GetCube) "None" (Variables|Default|GetSelf%20Location) "0, 0, 0" "1.000000,1.000000,1.000000" "KeepWorldPosition"))
  (Variables|Default|SetLightParticle _returnvalue)
  (Class|ParticleSystemComponent|SetBeamSourcePoint (Variables|Default|GetLightParticle) 0 (Variables|Default|GetSelf%20Location))
  (Class|ParticleSystemComponent|SetBeamEndPoint (Variables|Default|GetLightParticle) 0 (Variables|Default|GetEnd%20Location))
  (Variables|Default|SetbPower true))

(event Custom|Activate%20Hit%20Actor
  ;[0.3787 0.6401 1 0.6 30] Activate the hit actor
  (Class|BPILightObject|Activate(Message) (Variables|Default|GetOut%20Hit%20Actor)))

(event EventBeginPlay
  (bind _returnvalue (Actor|GetActorOfClass "/Game/EOTA/Blueprints/BP_WidgetManager.BP_WidgetManager_C"))
  (Variables|Default|SetAS%20BP%20Widget%20Manager _returnvalue)
  (CallFunction|SetupLocation))

(event EventInteracted
  ;[0.3787 0.6401 1 0.6 30] When interacted from the player, test for an object in front
  (if (and (Variables|Default|GetCanInteract) (not (Variables|Default|GetbPower)))
    (CallFunction|TestforTarget)))

(event EventHideInteractUI
  ;[0.3787 0.6401 1 0.6 30] Hide the interact UI
  (Class|BPIHUD|HideInteractUI(Message) (Variables|Default|GetAS%20BP%20Widget%20Manager)))

(fn ConstructionScript)

(fn SetupLocation
  (bind _particle_spawnpoint (Variables|Default|GetParticle%20Spawnpoint))
  (bind _output_get (Variables|Default|SetSelf%20Location (Transformation|GetWorldLocation _particle_spawnpoint)))
  (Variables|Default|SetEnd%20Location (+ _output_get (* (Math|Vector|GetForwardVector _particle_spawnpoint) (Variables|Default|GetTest%20Distance)))))

(fn SetActorLocation
  (bind _particle_spawnpoint (Variables|Default|GetParticle%20Spawnpoint))
  (Variables|Default|SetEnd%20Location (+ (Transformation|GetWorldLocation _particle_spawnpoint) (* (Math|Vector|GetForwardVector _particle_spawnpoint) (Variables|Default|GetOut%20Hit%20Distance)))))