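; BP_Crystal is a rotatable light-relay puzzle crystal that emits a beam when powered and passes activation to what it hits.
; A forward trace finds the hit actor, then repeated traces shorten the beam's length until it stops just before that actor.
; When interacted with in range, it rotates, clears its beam, deactivates the hit actor, retraces and reactivates if powered.
; Its trigger sphere also toggles the knight's HUD prompt.
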(event OnComponentBeginOverlap(Triggersphere)
  (params (OverlappedComponent :type Primitive%20Component%20Object%20Reference) (OtherActor :type Actor%20Object%20Reference) (OtherComp :type Primitive%20Component%20Object%20Reference) (OtherBodyIndex :type Integer) (bFromSweep :type Boolean) (SweepResult :type Hit%20Result%20Structure%20%28by%20ref%29))
  ;[0.3787 0.6401 1 0.6 30] When inside self collision trigger, set interact to true
  (bind _output_get (Variables|Default|SetOverlap%20Actor OtherActor))
  (Variables|Default|SetCanInteract true)
  (if (and (== _output_get (Variables|Default|GetBP%20Knight%20Actor)) (Variables|Default|GetCanInteract))
    (Class|BPIHUD|ShowHUD(Message) (Variables|Default|GetBP%20Widget%20Manager) (Variables|Default|GetHUD%20Message))))

(event OnComponentEndOverlap(Triggersphere)
  (params (OverlappedComponent :type Primitive%20Component%20Object%20Reference) (OtherActor :type Actor%20Object%20Reference) (OtherComp :type Primitive%20Component%20Object%20Reference) (OtherBodyIndex :type Integer))
  ;[0.3787 0.6401 1 0.6 30] When outside self collision trigger, set interact to false
  (bind _output_get (Variables|Default|SetOverlap%20Actor OtherActor))
  (Variables|Default|SetCanInteract false)
  (if (== _output_get (Variables|Default|GetBP%20Knight%20Actor))
    (Class|BPIHUD|HideHUD(Message) (Variables|Default|GetBP%20Widget%20Manager))))

(event Custom|Set%20Light%20Points
  ;[0.3787 0.6401 1 0.6 30] Set the particle start point and end point
  (Class|ParticleSystemComponent|SetBeamSourcePoint (Variables|Default|GetLight%20Particle) 0 (Variables|Default|GetSelf%20Location))
  (Class|ParticleSystemComponent|SetBeamEndPoint (Variables|Default|GetLight%20Particle) 0 (Variables|Default|GetEnd%20Location)))

(event Custom|Reset%20Light%20Source
  (bind _light_point (Variables|Default|GetLight%20point))
  ;[1 1 1 0.5 30] Set self and end location to the default values
  (bind _output_get (Variables|Default|SetSelf%20Location (Transformation|GetWorldLocation _light_point)))
  (Variables|Default|SetEnd%20Location (+ _output_get (* (Math|Vector|GetForwardVector _light_point) 2e+03))))

(event Custom|Activate%20Hit%20Actor
  ;[1 1 1 0.5 30] Activate the hit actor
  (Class|BPILightObject|Activate(Message) (Variables|Default|GetOut%20Hit%20Actor)))

(event Custom|Set%20Hit%20Location
  ;[0.3787 0.6401 1 0.6 30] Set end hit actor location
  (Variables|Default|SetEnd%20Hit%20Location (Transformation|GetActorLocation (Variables|Default|GetOut%20Hit%20Actor))))

(event Custom|Destroy%20All%20Particles
  ;[0.3787 0.6401 1 0.6 30] Destroy all particles inside the list if greater than 0 and reset the light source locations
  (CallFunction|ResetLightSource)
  (if (> (Utilities|Array|Length (Variables|Default|GetLight%20Particles)) 0)
    (Components|DestroyComponent (Variables|Default|GetLight%20Particles))
    (Utilities|Array|Clear (Variables|Default|GetLight%20Particles))))

(event Custom|Test%20For%20Target
  ;[0.6302 0.6009 0.2096 0.6 30] Line trace from self to forward, seeing if the correct object is in front
  (bind _outhit (Collision|LineTraceByChannel (Variables|Default|GetSelf%20Location) (Variables|Default|GetEnd%20Location) "TraceTypeQuery1" false 0 "ForDuration" true "(R=1.000000,G=0.000000,B=0.000000,A=1.000000)" "(R=0.000000,G=1.000000,B=0.000000,A=1.000000)" 2.0))
  (bind _output_get (Variables|Default|SetOut%20Hit%20Actor (.hitactor _outhit)))
  (Utilities|IsValid _output_get
    (:Is%20Valid
      (if (Actor|ActorHasTag _output_get "Light Obj")
        (bind _output_get_2 (Variables|Boolean|SetbLineMatch true))
        (Variables|Boolean|SetbLineHit _output_get_2)
        (CallFunction|FindActorLocation)
        (else
          (Variables|Boolean|SetbLineMatch false)
          (Variables|Boolean|SetbLineHit true)
          (CallFunction|FindActorLocation))))
    (:Is%20Not%20Valid
      (Variables|Boolean|SetbLineHit false))))

(event Custom|Find%20Actor%20Location
  (bind _light_point (Variables|Default|GetLight%20point))
  ;[0.3787 0.6401 1 0.6 30] Find the location right before the hit actor and set end location to the new location
  (Variables|Default|SetEnd%20Location%20Length 1e+03)
  (while (Variables|Boolean|GetbTraceHit)
    (bind _output_get (Variables|Default|SetEnd%20Location (+ (Transformation|GetWorldLocation _light_point) (* (Math|Vector|GetForwardVector _light_point) (Variables|Default|GetEnd%20Location%20Length)))))
    (bind _outhit (Collision|LineTraceByChannel (Variables|Default|GetSelf%20Location) _output_get "TraceTypeQuery1" false 0 "None"))
    (Utilities|IsValid (.hitactor _outhit)
      (:Is%20Valid
        (Variables|Boolean|SetbTraceHit true)
        (Variables|Default|SetEnd%20Location%20Length (- (Variables|Default|GetEnd%20Location%20Length) 5.0)))
      (:Is%20Not%20Valid
        (Variables|Boolean|SetbTraceHit false))))
  (Variables|Boolean|SetbTraceHit true)
  (Development|PrintString (Utilities|GetDisplayName (Variables|Default|GetOut%20Hit%20Actor))))

(event Custom|Deactivate%20Hit%20Actor
  (Class|BPILightObject|Deactivate(Message) (Variables|Default|GetOut%20Hit%20Actor)))

(event Custom|Set%20End%20Location
  (Variables|Default|SetEnd%20Location (+ (* (Variables|Default|GetSelf%20Location) "0.000000,0.000000,1.000000") (* (Variables|Default|GetEnd%20Hit%20Location) "1.000000,1.000000,0.000000"))))

(event EventBeginPlay
  (bind _light_point (Variables|Default|GetLight%20point))
  (bind _output_get (Variables|Default|SetSelf%20Location (Transformation|GetWorldLocation _light_point)))
  (Variables|Default|SetEnd%20Location (+ _output_get (* (Math|Vector|GetForwardVector _light_point) (Variables|Default|GetEnd%20Location%20Length))))
  (CallFunction|TestforTarget)
  (bind _returnvalue (Actor|GetActorOfClass "/Game/EOTA/Blueprints/Character/Knight/BP_Knight_FP.BP_Knight_FP_C"))
  (Variables|Default|SetBP%20Knight%20Actor _returnvalue)
  (bind _returnvalue_2 (Actor|GetActorOfClass "/Game/EOTA/Blueprints/BP_WidgetManager.BP_WidgetManager_C"))
  (Variables|Default|SetBP%20Widget%20Manager _returnvalue_2)
  (bind _outactors (Actor|GetAllActorsOfClass "BP_Crystal_C"))
  (Variables|Default|SetBP%20Crystal%20Actors _outactors)
  (bind _outactors_2 (Actor|GetAllActorswithTag "Light Obj"))
  (Variables|Default|SetLight%20Obj%20Actors _outactors_2))

(event EventCheckPower
  (Class|BPILightObject|CheckPower(Message) (Variables|Default|GetLight%20Obj%20Actors))
  (if (not (Variables|Boolean|GetbPower))
    (CallFunction|DestroyAllParticles)))

(event EventInteracted
  ;[0.6302 0.6009 0.2096 0.6 30] Interface event from Knight_FP when interacted will deactivate the light from the hit actor and rotate the crystal 35 degrees
  (if (Variables|Default|GetCanInteract)
    (bind _output_get (Variables|Default|SetSelf%20Rotation (Transformation|GetWorldRotation (Variables|Default|GetDefaultSceneRoot))))
    (Transformation|SetWorldRotation (Variables|Default|GetDefaultSceneRoot) (Math|Rotator|CombineRotators _output_get "0.000000,45.000000,0.000000") false false)
    (CallFunction|DestroyAllParticles)
    (CallFunction|DeactivateHitActor)
    (CallFunction|TestforTarget)
    (if (Variables|Boolean|GetbPower)
      (CallFunction|Activate))))

(event EventActivate
  ;[0.3787 0.6401 1 0.6 30] Interface event from Light Emitter will spawn the particle emitter at self location and adds the particle to the light particle list
  (Variables|Boolean|SetbPower true)
  (Utilities|FlowControl|Delay 1.0)
  (bind _returnvalue (Effects|SpawnEmitterAttached "/Game/EOTA/Niagara/CP_LightBeam_Crystal.CP_LightBeam_Crystal" (Variables|Default|GetLight%20point) "None" (Variables|Default|GetSelf%20Location) "0, 0, 0" "1.000000,1.000000,1.000000" "KeepWorldPosition" false))
  (bind _output_get (Variables|Default|SetLight%20Particle _returnvalue))
  (Utilities|IsValid _output_get
    (:Is%20Valid
      (Utilities|Array|Add (Variables|Default|GetLight%20Particles) _output_get)
      (Class|ParticleSystemComponent|SetBeamSourcePoint (Variables|Default|GetLight%20Particle) 0 (Variables|Default|GetSelf%20Location))
      (Class|ParticleSystemComponent|SetBeamEndPoint (Variables|Default|GetLight%20Particle) 0 (Variables|Default|GetEnd%20Location))
      (if (Variables|Boolean|GetbPower)
        (CallFunction|ActivateHitActor)))))

(fn ConstructionScript)