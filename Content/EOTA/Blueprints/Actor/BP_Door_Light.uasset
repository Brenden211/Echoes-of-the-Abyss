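; BP_Door_Light is a door actor that opens and closes by toggling its Doorway component rather than animating it.
; Its ToggleDoor event passes an active flag to a function of the same name.
; When active, that function hides the Doorway in game and disables its collision; when inactive, it shows it and restores query and physics collision.
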(event Custom|Event%20Toggle%20Door
  (params (IsActive :type Boolean))
  ;[0.3787 0.6401 1 1 30] Toggle the door
  (CallFunction|ToggleDoor IsActive))

(fn ConstructionScript)

(fn ToggleDoor
  (params (IsActive :type Boolean))
  (if IsActive
    (Collision|SetCollisionEnabled (Variables|Default|GetDoorway) "NoCollision")
    (Development|SetHiddeninGame (Variables|Default|GetDoorway) true false)
    (else
      (Collision|SetCollisionEnabled (Variables|Default|GetDoorway) "QueryAndPhysics")
      (Development|SetHiddeninGame (Variables|Default|GetDoorway) false false))))