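; BP_Lever is an interactable dungeon lever that toggles the doors registered to it through SetDoortoLever.
; Overlapping its box lets BP_Knight_FP interact and binds to the player's interact event, with a flag cleared on exit.
; Interaction flip-flops a timeline forward or backward to rotate the handle.
; A DoOnce on timeline updates, reset on finish, passes each stored door to BP_Dungeon_CH_Switch's LeverToggleDoor.
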(event OnComponentBeginOverlap(InteractBox)
  (params (OverlappedComponent :type Primitive%20Component%20Object%20Reference) (OtherActor :type Actor%20Object%20Reference) (OtherComp :type Primitive%20Component%20Object%20Reference) (OtherBodyIndex :type Integer) (bFromSweep :type Boolean) (SweepResult :type Hit%20Result%20Structure%20%28by%20ref%29))
  ;[0.3787 0.6401 1 1 30] When the player enters the collision box of the lever, they can interact
  (bind _asbp_knight_fp (Utilities|Casting|CastToBP_Knight_FP OtherActor))
  (Variables|Default|SetCanInteract true)
  (EventDispatchers|BindEventtoPlayerInteracted _asbp_knight_fp (EventDispatchers|CreateEvent :!event Custom|Toggle%20Lever)))

(event OnComponentEndOverlap(InteractBox)
  (params (OverlappedComponent :type Primitive%20Component%20Object%20Reference) (OtherActor :type Actor%20Object%20Reference) (OtherComp :type Primitive%20Component%20Object%20Reference) (OtherBodyIndex :type Integer))
  ;[0.3787 0.6401 1 1 30] When the player leaves the collision box of the lever, they can not interact with it
  (Utilities|Casting|CastToBP_Knight_FP OtherActor)
  (Variables|Default|SetCanInteract false))

(event Custom|Toggle%20Lever
  ;[0.3787 0.6401 1 1 30] If the player can interact, the event binds to this event when they press the interact button and will toggle the lever is active state
  (if (Variables|Default|GetCanInteract)
    (Utilities|FlowControl|FlipFlop
      (:A
        (bind _flip_lever (Timeline|Rotate%20Lever Play)
          (:Update
            (Transformation|SetRelativeRotation (Variables|Default|GetHandle) (Math|Rotator|MakeRotator (* _flip_lever 9e+01) 0.0 0.0) false false)
            (Utilities|FlowControl|DoOnce false :!label _label
              (:Completed
                (CallFunction|ToggleDoor))))
          (:Finished
            (goto _label Reset))))
      (:B
        (Timeline|Rotate%20Lever Reverse)))))

(event Custom|Set%20Door%20to%20Lever
  (params (In%20Door :type Actor%20Object%20Reference))
  (Utilities|Array|Add (Variables|Default|GetDoor) In%20Door))

(event Custom|Toggle%20Door
  (bind _returnvalue (Actor|GetActorOfClass "/Game/EOTA/Blueprints/Dungeon/MainRoom/Challenge/BP_Dungeon_CH_Switch.BP_Dungeon_CH_Switch_C"))
  (for _array_element (Variables|Default|GetDoor)
    (Default|LeverToggleDoor _returnvalue _array_element)
    (Development|PrintString "A door changed...")))

(fn ConstructionScript)