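; Light receiver actor that opens and closes a dungeon door according to whether it receives power.
; Power interface events Activate and Deactivate set IsPowered, swap the cube between green and dull materials, and toggle the BP_Dungeon_CH_Light found by class lookup at BeginPlay.
; Activation applies after a short delay, deactivation is immediate, and a receiver that starts powered activates itself.
; GetPower always returns false, independent of IsPowered.
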(event EventBeginPlay
  (bind _returnvalue (Actor|GetActorOfClass "/Game/EOTA/Blueprints/Actor/Dungeon/Rooms/Challenge/BP_Dungeon_CH_Light.BP_Dungeon_CH_Light_C"))
  (Variables|Default|SetAs%20BP%20Dungeon%20CH%20Light _returnvalue)
  (if (Variables|Default|GetIsPowered)
    (CallFunction|Activate)))

(event EventActivate
  (params (In%20Activated%20Actor :type Actor%20Object%20Reference))
  (bind _as_bp_dungeon_ch_light (Variables|Default|GetAs%20BP%20Dungeon%20CH%20Light))
  ;[0.3787 0.6401 1 0.6 30] Called from the BPI interface when recieving power to activate the door
  (Variables|Default|SetIsPowered true)
  (Utilities|FlowControl|Delay 0.8)
  (Rendering|Material|SetMaterial (Variables|Default|GetCube) 0 "/Game/EOTA/Materials/M_Light_Green.M_Light_Green")
  (Utilities|IsValid _as_bp_dungeon_ch_light
    (:Is%20Valid
      (Default|EventToggleDoor _as_bp_dungeon_ch_light true))))

(event EventDeactivate
  (bind _as_bp_dungeon_ch_light (Variables|Default|GetAs%20BP%20Dungeon%20CH%20Light))
  ;[0.3787 0.6401 1 0.6 30] Called from the BPI interface when not recieving power to deactivate and close the door
  (Variables|Default|SetIsPowered false)
  (Rendering|Material|SetMaterial (Variables|Default|GetCube) 0 "/Game/EOTA/Materials/M_Light_Dull.M_Light_Dull")
  (Utilities|IsValid _as_bp_dungeon_ch_light
    (:Is%20Valid
      (Default|EventToggleDoor _as_bp_dungeon_ch_light false))))

(fn ConstructionScript)

(fn GetPower
  (return false))