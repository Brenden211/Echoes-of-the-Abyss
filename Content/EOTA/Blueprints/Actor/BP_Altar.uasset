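; BP_Altar is an interactable altar where the player places carried relics into four slots.
; Overlapping its collision as the first-person knight while holding a relic shows a prompt through the widget manager.
; Interacted spawns the relic actor at the slot matching the game instance's inventory index, marks it in AltarInventory, then clears the held relic and its UI.
; HasAllRelic reports whether every inventory entry is filled.
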(event OnComponentBeginOverlap(InteractCollision)
  (params (OverlappedComponent :type Primitive%20Component%20Object%20Reference) (OtherActor :type Actor%20Object%20Reference) (OtherComp :type Primitive%20Component%20Object%20Reference) (OtherBodyIndex :type Integer) (bFromSweep :type Boolean) (SweepResult :type Hit%20Result%20Structure%20%28by%20ref%29))
  (bind _output_get (Variables|Default|SetOverlap%20Actor OtherActor))
  (Variables|Default|SetIsOverlap true)
  (if (Math|Boolean|ANDBoolean (== _output_get (Variables|Default|GetTarget%20Actor)) (Variables|Default|GetCanInteract) (Variables|/Game/EOTA/Blueprints/BP_MainGameInstance.BP_MainGameInstance_C|GetHoldingRelic (Variables|Default|GetAs%20BP%20Main%20Game%20Instance)))
    (Class|BPIHUD|ShowInteractUI(Message) (Variables|Default|GetAS%20BP%20Widget%20Manager) (Variables|Default|GetHUD%20Message))))

(event OnComponentEndOverlap(InteractCollision)
  (params (OverlappedComponent :type Primitive%20Component%20Object%20Reference) (OtherActor :type Actor%20Object%20Reference) (OtherComp :type Primitive%20Component%20Object%20Reference) (OtherBodyIndex :type Integer))
  (bind _output_get (Variables|Default|SetOverlap%20Actor OtherActor))
  (Variables|Default|SetIsOverlap false)
  (if (and (== _output_get (Variables|Default|GetTarget%20Actor)) (Variables|Default|GetCanInteract))
    (Class|BPIHUD|HideInteractUI(Message) (Variables|Default|GetAS%20BP%20Widget%20Manager))))

(event EventBeginPlay
  (bind _asbp_main_game_instance (Utilities|Casting|CastToBP_MainGameInstance (Game|GetGameInstance)))
  (Variables|Default|SetAs%20BP%20Main%20Game%20Instance _asbp_main_game_instance)
  (bind _returnvalue (Actor|GetActorOfClass "/Game/EOTA/Blueprints/Character/Knight/BP_Knight_FP.BP_Knight_FP_C"))
  (Variables|Default|SetTarget%20Actor _returnvalue)
  (bind _returnvalue_2 (Actor|GetActorOfClass "/Game/EOTA/Blueprints/BP_WidgetManager.BP_WidgetManager_C"))
  (Variables|Default|SetAS%20BP%20Widget%20Manager _returnvalue_2))

(event EventInteracted
  (bind _as_bp_main_game_instance (Variables|Default|GetAs%20BP%20Main%20Game%20Instance))
  (bind _inventoryindex (Variables|/Game/EOTA/Blueprints/BP_MainGameInstance.BP_MainGameInstance_C|GetInventoryIndex _as_bp_main_game_instance))
  (if (and (Variables|/Game/EOTA/Blueprints/BP_MainGameInstance.BP_MainGameInstance_C|GetHoldingRelic (Variables|Default|GetAs%20BP%20Main%20Game%20Instance)) (Variables|Default|GetIsOverlap))
    (CallFunction|PlaceRelic _inventoryindex)
    (CallFunction|UpdateAltarInventory _inventoryindex)
    (Default|ToggleRelicUI (Variables|Default|GetAS%20BP%20Widget%20Manager) false)
    (Default|SetRelicType (Variables|Default|GetAs%20BP%20Main%20Game%20Instance) "NewEnumerator6" false)
    (else
      (Development|PrintString "No Relic"))))

(event EventHideInteractUI
  ;[0.3787 0.6401 1 0.6 30] Hide the interact UI
  (Class|BPIHUD|HideInteractUI(Message) (Variables|Default|GetAS%20BP%20Widget%20Manager)))

(fn ConstructionScript)

(fn UpdateAltarInventory
  (params (Relic%20Index :type Integer))
  (Utilities|Array|SetArrayElem (Variables|Default|GetAltar%20Inventory) Relic%20Index true))

(fn PlaceRelic
  (params (Relic%20Index :type Integer))
  (bind _output_get (LocalVariables|SetRelicIndex Relic%20Index))
  (Utilities|FlowControl|Sequence
    (:then_0
      (switch int _output_get
        (:0
          (LocalVariables|SetSlot%20Location (Transformation|GetWorldTransform (Variables|Default|GetRelic%20Slot1))))
        (:1
          (LocalVariables|SetSlot%20Location (Transformation|GetWorldTransform (Variables|Default|GetRelic%20Slot2))))
        (:2
          (LocalVariables|SetSlot%20Location (Transformation|GetWorldTransform (Variables|Default|GetRelic%20Slot3))))
        (:3
          (LocalVariables|SetSlot%20Location (Transformation|GetWorldTransform (Variables|Default|GetRelic%20Slot4))))))
    (:then_1
      (Game|SpawnActorfromClass (Utilities|Array|Get(acopy) (Variables|Default|GetRelic%20Actors) _output_get) (LocalVariables|GetSlot%20Location) "Undefined" "MultiplyWithRoot" 0 0))))

(fn HasAllRelic
  (for _array_element (Variables|Default|GetAltar%20Inventory)
    (if (== _array_element false)
      (LocalVariables|SetHasRelics false)))
  (return (LocalVariables|GetHasRelics)))