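; Skelzomb enemy character that detects pawns by sight and passes them to its AI Blackboard as TargetActor.
; PawnSensing pauses by zeroing its interval after a sighting, until ResetPawnSensing restores it, with optional debug cone and sphere drawing.
; At BeginPlay, IgnorePlayer can switch sensing off and LookPretty sets the Blackboard Idle flag.
; TakeDamage forwards hits to the WBCHealth component, and Death destroys the actor.
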(event OnSeePawn(PawnSensing)
  (params (Pawn :type Pawn%20Object%20Reference))
  (Variables|Default|SetSensedPawn Pawn)
  (CallFunction|ShowDebug (Variables|Debug|GetCone%20from%20Enemy) (Variables|Debug|GetSphere%20from%20Target))
  (AI|Components|Blackboard|SetValueasObject (AI|GetBlackboard 0) (Utilities|Name|MakeLiteralName "TargetActor") (Variables|Default|GetSensedPawn))
  (Class|PawnSensingComponent|SetSensingInterval (Variables|Default|GetPawnSensing) 0.0))

(event Custom|Reset%20Pawn%20Sensing
  (Class|PawnSensingComponent|SetSensingInterval (Variables|Default|GetPawnSensing) 0.1)
  (Development|PrintString "reset pawn sensing"))

(event Custom|Show%20Debug
  (params (Cone :type Boolean) (Sphere :type Boolean))
  (if Cone
    (CallFunction|DrawDebugCone))
  (if Sphere
    (CallFunction|DrawDebugSphere)))

(event EventTakeDamage
  (params (Hits :type Integer))
  (Default|UpdateHealth (Variables|Default|GetWBC_Health) (Math|Conversions|ToFloat(Integer) Hits)))

(event EventBeginPlay
  (CallFunction|CheckIgnorePlayer)
  (CallFunction|CheckIdle))

(event EventDeath
  (Actor|DestroyActor))

(fn ConstructionScript)

(fn DrawDebugCone
  (bind _pawnsensing (Variables|Default|GetPawnSensing))
  (bind _returnvalue (Class|PawnSensingComponent|GetPeripheralVisionAngle _pawnsensing))
  (Class|KismetSystemLibrary|DrawDebugConeinDegrees (Class|CharacterMovementComponent|GetLastUpdateLocation (Variables|Character|GetCharacterMovement)) (Math|Rotator|GetRotationXVector (Class|CharacterMovementComponent|GetLastUpdateRotation (Variables|Character|GetCharacterMovement))) (Variables|/Script/AIModule.PawnSensingComponent|GetSightRadius _pawnsensing) _returnvalue _returnvalue 12 "(R=1.000000,G=1.000000,B=1.000000,A=1.000000)" 3.0 0.0))

(fn DrawDebugSphere
  (Rendering|Debug|DrawDebugSphere (Transformation|GetActorLocation (Variables|Default|GetSensedPawn)) 5e+01 12 "(R=1.000000,G=0.286837,B=0.270833,A=1.000000)" 3.0))

(fn CheckIgnorePlayer
  (bind _pawnsensing (Variables|Default|GetPawnSensing))
  (if (Variables|Debug(beforeplay)|GetIgnore%20Player)
    (Class|PawnSensingComponent|SetSensingInterval _pawnsensing 0.0)
    (else
      (Class|PawnSensingComponent|SetSensingInterval _pawnsensing 0.1))))

(fn CheckIdle
  (if (Variables|Debug(beforeplay)|GetLook%20Pretty)
    (AI|Components|Blackboard|SetValueasBool (AI|GetBlackboard 0) (Utilities|Name|MakeLiteralName "Idle") true)
    (else
      (AI|Components|Blackboard|SetValueasBool (AI|GetBlackboard 0) (Utilities|Name|MakeLiteralName "Idle") false))))