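; Dungeon manager that assembles the level at BeginPlay from a start room, hallway, central hub and up to four zones.
; Fixed pieces chain through exit components; zones attach to hub exits matched by display name, each receiving a room goal.
; Each SpawnZone call records a generation time and advances one zone.
; After the fourth, it prints stats, triggers relic altars and light emitters, then notifies the game instance; door-frame and exit-closing events are stubs.
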(event Custom|Spawn%20Start%20Room
  ;[0.3787 0.6401 1 0.6 30] Spawn start room
  (bind _returnvalue (Game|SpawnActorfromClass "/Game/EOTA/Blueprints/Actor/Dungeon/Rooms/Starting/BP_Dungeon_StartRoom.BP_Dungeon_StartRoom_C" (Transformation|GetWorldTransform (Variables|Components|GetDefaultSceneRoot)) "AlwaysSpawn" "MultiplyWithRoot" 0 0))
  (bind _output_get (Variables|Components|SetLatest%20Exit (Components|GetChildComponent (Variables|/Game/EOTA/Blueprints/Actor/Dungeon/BP_Dungeon_MasterRoom.BP_Dungeon_MasterRoom_C|GetExit%20Folder _returnvalue) 0)))
  (Utilities|Array|Add (Variables|ComponentList|GetExit%20List) _output_get))

(event Custom|Spawn%20Start%20Hallway
  ;[0.3787 0.6401 1 0.6 30] Spawn start hallway
  (bind _returnvalue (Game|SpawnActorfromClass "/Game/EOTA/Blueprints/Actor/Dungeon/Rooms/Starting/BP_Dungeon_StartHallway.BP_Dungeon_StartHallway_C" (Transformation|GetWorldTransform (Variables|Components|GetLatest%20Exit)) "AlwaysSpawn" "MultiplyWithRoot" 0 0))
  (bind _output_get (Variables|Components|SetLatest%20Exit (Components|GetChildComponent (Variables|/Game/EOTA/Blueprints/Actor/Dungeon/BP_Dungeon_MasterRoom.BP_Dungeon_MasterRoom_C|GetExit%20Folder _returnvalue) 0)))
  (Utilities|Array|Add (Variables|ComponentList|GetExit%20List) _output_get))

(event Custom|Spawn%20Zone%204
  ;[0.3787 0.6401 1 0.6 30] Spawn zone 4
  (CallFunction|SetZoneExit (Variables|ComponentList|GetCentralHubExits) (Variables|String|GetZone4%20Actor%20Name))
  (bind _returnvalue (Game|SpawnActorfromClass "/Game/EOTA/Blueprints/Dungeon/BP_Zone4.BP_Zone4_C" (Transformation|GetWorldTransform (Variables|Components|GetZone%20Exit)) "AlwaysSpawn" "MultiplyWithRoot" 0 (Variables|Zone4|GetZone4%20Rooms) "Zone 4" 0))
  (Variables|Default|SetZone4 _returnvalue)
  (Utilities|Array|Add (Variables|List|GetZone%20Rooms%20List) (Variables|Zone4|GetZone4%20Rooms)))

(event Custom|Spawn%20Zone%201
  ;[0.3787 0.6401 1 0.6 30] Spawn zone 1
  (CallFunction|SetZoneExit (Variables|ComponentList|GetCentralHubExits) (Variables|String|GetZone1%20Actor%20Name))
  (bind _returnvalue (Game|SpawnActorfromClass "/Game/EOTA/Blueprints/Dungeon/BP_Zone1.BP_Zone1_C" (Transformation|GetWorldTransform (Variables|Components|GetZone%20Exit)) "AlwaysSpawn" "MultiplyWithRoot" 0 (Variables|Zone1|GetZone1%20Rooms) "ZONE 1" 0))
  (Variables|Default|SetZone1 _returnvalue)
  (Utilities|Array|Add (Variables|List|GetZone%20Rooms%20List) (Variables|Zone1|GetZone1%20Rooms)))

(event Custom|Spawn%20Relics
  (Default|SpawnRelicAltar (Variables|Default|GetZone1) "NewEnumerator0")
  (Default|SpawnRelicAltar (Variables|Default|GetZone2) "NewEnumerator1")
  (Default|SpawnRelicAltar (Variables|Default|GetZone3) "NewEnumerator2")
  (Default|SpawnRelicAltar (Variables|Default|GetZone4) "NewEnumerator5"))

(event Custom|Spawn%20Light%20Emitter
  (Default|SpawnLightEmitter (Variables|Default|GetZone1))
  (Default|SpawnLightEmitter (Variables|Default|GetZone2))
  (Default|SpawnLightEmitter (Variables|Default|GetZone3))
  (Default|SpawnLightEmitter (Variables|Default|GetZone4)))

(event Custom|Event%20Spawn%20Zone%20Items
  (CallFunction|PrintDungeonDetails)
  (CallFunction|SpawnRelics)
  (CallFunction|SpawnLightEmitter)
  (CallFunction|DungeonReady))

(event Custom|Spawn%20Door%20Frames
  ;[0.3787 0.6401 1 0.6 30] Spawn the door frame at each exit
)

(event Custom|Spawn%20Central%20Hub
  ;[0.3787 0.6401 1 0.6 30] Spawn central hub then set the hub's exits
  (bind _returnvalue (Game|SpawnActorfromClass "/Game/EOTA/Blueprints/Actor/Dungeon/Rooms/Starting/BP_Dungeon_CentralHub.BP_Dungeon_CentralHub_C" (Transformation|GetWorldTransform (Variables|Components|GetLatest%20Exit)) "AlwaysSpawn" "MultiplyWithRoot" 0 0))
  (Utilities|Array|AppendArray (Variables|ComponentList|GetExit%20List) (Components|GetChildrenComponents (Variables|/Game/EOTA/Blueprints/Actor/Dungeon/BP_Dungeon_MasterRoom.BP_Dungeon_MasterRoom_C|GetExit%20Folder _returnvalue) false))
  (Variables|ComponentList|SetCentralHubExits (Components|GetChildrenComponents (Variables|/Game/EOTA/Blueprints/Actor/Dungeon/BP_Dungeon_MasterRoom.BP_Dungeon_MasterRoom_C|GetExit%20Folder _returnvalue) false)))

(event Custom|Spawn%20Zone
  (params (Input%20Zone%20Seconds :type Integer))
  ;[0.1329 0.2482 0.5208 0.6 30] Spawns each zone from index value inside the level and set how long that zone takes to generate
  (bind _output_get (Variables|Default|SetZone%20Seconds Input%20Zone%20Seconds))
  (Utilities|Array|Add (Variables|List|GetZone%20Time%20List) _output_get)
  (switch int (Variables|Default|GetZone%20Index)
    (:0
      (if (Variables|Zone1|GetbSpawnZone1)
        (CallFunction|SpawnZone1)
        (Math|Integer|IncrementInt (Variables|Default|GetZone%20Index) :!label _label)))
    (:1
      (if (Variables|Zone2|GetbSpawnZone2)
        (CallFunction|SpawnZone2)
        (Development|PrintString "-----------")
        (goto _label)))
    (:2
      (if (Variables|Zone3|GetbSpawnZone3)
        (CallFunction|SpawnZone3)
        (Development|PrintString "-----------")
        (goto _label)))
    (:3
      (if (Variables|Zone4|GetbSpawnZone4)
        (CallFunction|SpawnZone4)
        (goto _label)))
    (:4
      (CallFunction|EventSpawnZoneItems))))

(event Custom|Close%20Exit
  ;[0.3787 0.6401 1 0.6 30] Close all exits that are not connected to any room.
)

(event Custom|Spawn%20Zone%202
  ;[0.3787 0.6401 1 0.6 30] Spawn zone 2
  (CallFunction|SetZoneExit (Variables|ComponentList|GetCentralHubExits) (Variables|String|GetZone2%20Actor%20Name))
  (bind _returnvalue (Game|SpawnActorfromClass "/Game/EOTA/Blueprints/Dungeon/BP_Zone2.BP_Zone2_C" (Transformation|GetWorldTransform (Variables|Components|GetZone%20Exit)) "AlwaysSpawn" "MultiplyWithRoot" 0 (Variables|Zone2|GetZone2%20Rooms) "Zone 2" 0))
  (Variables|Default|SetZone2 _returnvalue)
  (Utilities|Array|Add (Variables|List|GetZone%20Rooms%20List) (Variables|Zone2|GetZone2%20Rooms)))

(event Custom|Print%20Dungeon%20Details
  (bind _printdungeonindex (Variables|Default|GetPrintDungeonIndex))
  ;[0.3787 0.6401 1 0.6 30] Print the details for the dungeon zones
  (while (Variables|Default|GetbPrintDungeon)
    (CallFunction|PrintZoneDetails (Utilities|Array|Get(acopy) (Variables|List|GetZone%20Rooms%20List) (Variables|Default|GetPrintDungeonIndex)) (Utilities|Array|Get(acopy) (Variables|List|GetZone%20Name%20List) (Variables|Default|GetPrintDungeonIndex)) (Utilities|Array|Get(acopy) (Variables|List|GetZone%20Time%20List) (Variables|Default|GetPrintDungeonIndex)))
    (Development|PrintString "----------" true true "(R=0.000000,G=0.660000,B=1.000000,A=1.000000)" 15.0)
    (Math|Integer|IncrementInt _printdungeonindex
      (:%20%20
        (if (>= _printdungeonindex (Variables|Default|GetZone%20Index%20Total))
          (Variables|Default|SetbPrintDungeon false))))))

(event Custom|Spawn%20Zone%203
  ;[0.3787 0.6401 1 0.6 30] Spawn zone 3
  (CallFunction|SetZoneExit (Variables|ComponentList|GetCentralHubExits) (Variables|String|GetZone3%20Actor%20Name))
  (bind _returnvalue (Game|SpawnActorfromClass "/Game/EOTA/Blueprints/Dungeon/BP_Zone3.BP_Zone3_C" (Transformation|GetWorldTransform (Variables|Components|GetZone%20Exit)) "AlwaysSpawn" "MultiplyWithRoot" 0 (Variables|Zone3|GetZone3%20Rooms) "Zone 3" 0))
  (Variables|Default|SetZone3 _returnvalue)
  (Utilities|Array|Add (Variables|List|GetZone%20Rooms%20List) (Variables|Zone3|GetZone3%20Rooms)))

(event Custom|Dungeon%20Ready
  ;[0.3787 0.6401 1 0.6 30] When dungeon is generated, call to game instance
  (Default|DungeonReady (Variables|Default|GetAs%20BP%20Main%20Game%20Instance))
  (Development|PrintString "DUNGEON READY" true true "(R=0.000000,G=1.000000,B=0.376976,A=0.600000)" 5.0))

(event EventBeginPlay
  (bind _asbp_main_game_instance (Utilities|Casting|CastToBP_MainGameInstance (Game|GetGameInstance)))
  (Variables|Default|SetAs%20BP%20Main%20Game%20Instance _asbp_main_game_instance)
  (CallFunction|SpawnStartRoom)
  (CallFunction|SpawnStartHallway)
  (CallFunction|SpawnCentralHub)
  (CallFunction|SpawnDoorFrames)
  (CallFunction|SpawnZone))

(fn ConstructionScript)

(fn SetZoneExit
  (params (Exits :type Array%20of%20Scene%20Component%20Object%20References) (Zone%20Name :type String))
  (for _array_element Exits
    (LocalVariables|SetExit _array_element)
    (if (Utilities|Enum|Equal(Enum) (Utilities|GetDisplayName _array_element) Zone%20Name)
      (Variables|Components|SetZone%20Exit (LocalVariables|GetExit)))))

(fn PrintZoneDetails
  (params (Zone%20Room%20Goal :type Integer%20%28by%20ref%29) (Zone%20Name :type String%20%28by%20ref%29) (Zone%20Time%20Seconds :type Integer%20%28by%20ref%29))
  (Development|PrintString (Utilities|String|Append Zone%20Name " CREATED: " (Utilities|String|ToString(Integer) Zone%20Room%20Goal)) true true "(R=0.493814,G=0.348958,B=1.000000,A=1.000000)" 15.0)
  (Development|PrintString (Utilities|String|Append Zone%20Name " COMPLETED: " (Utilities|String|ToString(Text) (Utilities|Text|FormatText (Utilities|Text|ToText(Integer) Zone%20Time%20Seconds)))) true true "(R=1.000000,G=0.945882,B=0.000000,A=1.000000)" 15.0))