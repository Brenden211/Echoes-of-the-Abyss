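; Procedural dungeon generator that builds a level at BeginPlay by attaching random rooms to open exits of a start room and previously placed rooms.
; Each room is overlap-tested after a delay and destroyed and retried on collision, with the last room drawn from a special list.
; On completion it walls unused exits and spawns random doors at connections.
; A looping watchdog timer reloads the test map if building exceeds a room-count-based time limit.
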(event Custom|Spawn%20Start%20Room
  ;[0.3787 0.6401 1 1 30] Spawn start room
  (bind _returnvalue (Game|SpawnActorfromClass "/Game/EOTA/Blueprints/Actor/Dungeon/Rooms/Starting/BP_Dungeon_StartRoom.BP_Dungeon_StartRoom_C" (Transformation|GetWorldTransform (Variables|Components|GetDefaultSceneRoot)) "AlwaysSpawn" "MultiplyWithRoot" 0 0))
  (Utilities|Array|AppendArray (Variables|Components|GetExit%20List) (Components|GetChildrenComponents (Variables|/Game/EOTA/Blueprints/Actor/Dungeon/BP_Dungeon_MasterRoom.BP_Dungeon_MasterRoom_C|GetExit%20Folder _returnvalue) false))
  (CallFunction|SpawnNextRoom))

(event Custom|Spawn%20Next%20Room
  ;[0.3787 0.6401 1 1 30] Selects a random exit from all the spawned rooms then spawns the next room at that exit. Also, sets the lastest room to the one that spawned.
  (Variables|Components|SetSelected%20Exit%20Point (.OutItem (Utilities|Array|Random (Variables|Components|GetExit%20List))))
  (bind _returnvalue (Game|SpawnActorfromClass (.OutItem (Utilities|Array|Random (Variables|ActorLists|GetRoom%20List))) (Transformation|GetWorldTransform (Variables|Components|GetSelected%20Exit%20Point)) "AlwaysSpawn" "MultiplyWithRoot" 0 0))
  (bind _asbp_dungeon_master_room (Utilities|Casting|CastToBP_Dungeon_MasterRoom _returnvalue))
  (Variables|Components|SetLatest%20Room _asbp_dungeon_master_room)
  (Utilities|FlowControl|Delay (Variables|Time|GetTime%20Between%20Rooms))
  (CallFunction|CheckforOverlap))

(event Custom|Add%20Overlapping%20Rooms%20to%20List
  ;[0.3787 0.6401 1 1 30] Add overlapping rooms to list
  (for _array_element (Components|GetChildrenComponents (Variables|/Game/EOTA/Blueprints/Actor/Dungeon/BP_Dungeon_MasterRoom.BP_Dungeon_MasterRoom_C|GetOverlap%20Folder (Variables|Components|GetLatest%20Room)) false)
    (bind _asbox_collision (Utilities|Casting|CastToBoxComponent _array_element))
    (Utilities|Array|AppendArray (Variables|Components|GetOverlaped%20List) (Class|PrimitiveComponent|GetOverlappingComponents _asbox_collision))))

(event Custom|Check%20for%20Overlap
  ;[0.3787 0.6401 1 1 30] Delete latest room if overlapping and keep spawning rooms. Also checks if all the rooms are spawned.
  (CallFunction|AddOverlappingRoomstoList)
  (if (Utilities|Array|IsNotEmpty (Variables|Components|GetOverlaped%20List))
    (Utilities|Array|Clear (Variables|Components|GetOverlaped%20List))
    (Actor|DestroyActor (Variables|Components|GetLatest%20Room))
    (CallFunction|SpawnNextRoom)
    (else
      (Utilities|Array|Clear (Variables|Components|GetOverlaped%20List))
      (Variables|Integers|SetRoom%20Total (- (Variables|Integers|GetRoom%20Total) 1))
      (Utilities|Array|RemoveItem (Variables|Components|GetExit%20List) (Variables|Components|GetSelected%20Exit%20Point))
      ;;[1 1 1 0.5] Add arrow to door list
      (Utilities|Array|Add (Variables|Components|GetDoor%20List) (Variables|Components|GetSelected%20Exit%20Point))
      (Utilities|Array|AppendArray (Variables|Components|GetExit%20List) (Components|GetChildrenComponents (Variables|/Game/EOTA/Blueprints/Actor/Dungeon/BP_Dungeon_MasterRoom.BP_Dungeon_MasterRoom_C|GetExit%20Folder (Variables|Components|GetLatest%20Room)) false))
      (if (> (Variables|Integers|GetRoom%20Total) 0)
        (if (== (Variables|Integers|GetRoom%20Total) 1)
          (Variables|ActorLists|SetRoom%20List (Variables|ActorLists|GetSpecial%20Room%20List))
          (else
            (Variables|ActorLists|SetRoom%20List (Variables|ActorLists|GetBase%20Room%20List))))
        (CallFunction|SpawnNextRoom)
        (else
          (Utilities|FlowControl|Delay (Variables|Time|GetClose%20Exits%20Delay))
          (CallFunction|CloseOpenedExits)
          (CallFunction|SpawnDoors)
          (Variables|Booleans|SetDungeonComplete true)
          (Utilities|Time|ClearandInvalidateTimerbyHandle (Variables|Timer|GetTimer%20Handle))
          (Development|PrintString "DUNGEON COMPLETE" true true "(R=1.000000,G=0.945882,B=0.000000,A=1.000000)" 5.0)
          (CallFunction|PrintDungeonRooms))))))

(event Custom|Spawn%20Doors
  ;[1 1 1 0.5 30] Spawn doors
  (for _array_element (Variables|Components|GetDoor%20List)
    (Game|SpawnActorfromClass (.OutItem (Utilities|Array|RandomFromStream (Variables|ActorLists|GetDoor%20Actor%20List) (Variables|Default|GetStream))) (Transformation|GetWorldTransform _array_element) "AlwaysSpawn" "MultiplyWithRoot" 0 0)))

(event Custom|Close%20Opened%20Exits
  ;[0.3787 0.6401 1 1 30] Close all the exits that are not connected to any room.
  (for _array_element (Variables|Components|GetExit%20List)
    (Game|SpawnActorfromClass "/Game/EOTA/Blueprints/Actor/Dungeon/Walls/BP_Dungeon_Exit_Wall.BP_Dungeon_Exit_Wall_C" (Transformation|GetWorldTransform _array_element) "AlwaysSpawn" "MultiplyWithRoot" 0 0)))

(event Custom|Start%20Dungeon%20Timer
  ;[0.3787 0.6401 1 1 30] Dungeon Timer
  (bind _returnvalue (Utilities|Time|SetTimerbyEvent (delegate Custom|Check%20for%20Dungeon%20Complete) 0.5 true))
  (Variables|Timer|SetTimer%20Handle _returnvalue))

(event Custom|Check%20for%20Dungeon%20Complete
  ;[0.3787 0.6401 1 1 30] Dungeon Timer
  (Development|PrintString "Running Timer")
  (if (>= (Utilities|Time|GetGameTimeinSeconds) (Variables|Timer|GetDungeon%20Build%20Time))
    (Game|OpenLevel(byName) "Map_ProceduralGenerationTest")))

(event EventBeginPlay
  (bind _output_get (Variables|Integers|SetRooms%20Spawned (Variables|Integers|GetRoom%20Total)))
  (Variables|Timer|SetDungeon%20Build%20Time (/ (Math|Conversions|ToFloat(Integer) _output_get) 2.0))
  (CallFunction|SpawnStartRoom)
  (CallFunction|StartDungeonTimer))

(fn ConstructionScript)

(fn PrintDungeonRooms
  (Development|PrintString (Utilities|String|Append "ROOMS GENERATED: " (Utilities|String|ToString(Integer) (Variables|Integers|GetRooms%20Spawned))) true true "(R=0.493814,G=0.348958,B=1.000000,A=1.000000)" 5.0))