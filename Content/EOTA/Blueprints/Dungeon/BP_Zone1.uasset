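; Procedurally builds one dungeon zone from the manager's zone exit: start hallway, light or switch challenge room, random rooms, then a relic room.
; Each room spawns at a random open exit and is destroyed and retried if its overlap boxes hit anything.
; Timeouts, exhausted exits or excessive failures reset the zone, with a level reload fallback.
; On completion it caps open exits, adds door frames and has BP_Dungeon_Manager spawn the next zone.
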(event Custom|Check%20Delete
  (bind _reset_current (Variables|ZoneDetails|GetReset%20Current))
  ;[0.3787 0.6401 1 0.6 30] Check for delete loop
  (if (> (Variables|ZoneDetails|GetDelete%20Current) (Variables|ZoneDetails|GetDelete%20Limit))
    (CallFunction|ResetZone)
    (Development|PrintString "DELETE RESET" true true "(R=0.630208,G=0.203505,B=0.203505,A=1.000000)" 4.0)
    (Math|Integer|IncrementInt _reset_current
      (:%20%20
        (if (>= _reset_current 5)
          (CallFunction|HardReset))))))

(event Custom|Spawn%20Random%20Room
  (bind _exit_list (Variables|Components|GetExit%20List))
  (bind _outitem (Utilities|Array|Random _exit_list))
  ;[0.2232 0.8963 1 0.5 30] Spawn a random room from the appropriate list
  (Utilities|FlowControl|Delay (Variables|Time|GetTime%20Between%20Rooms))
  (Utilities|IsValid _outitem
    (:Is%20Valid
      (bind _output_get (Variables|Components|SetSelected%20Exit%20Point _outitem))
      (bind _returnvalue (Game|SpawnActorfromClass (.OutItem (Utilities|Array|Random (Variables|RoomLists|GetRoom%20List))) (Transformation|GetWorldTransform _output_get) "AlwaysSpawn" "MultiplyWithRoot" 0 0))
      (bind _asbp_dungeon_master_room (Utilities|Casting|CastToBP_Dungeon_MasterRoom _returnvalue))
      (bind _output_get_2 (Variables|Components|SetLatest%20Room _asbp_dungeon_master_room))
      (Utilities|Array|Add (Variables|Components|GetGenerated%20List) _output_get_2)
      (CallFunction|AddOverlapRooms))))

(event Custom|Set%20Room
  ;[0.3787 0.6401 1 0.6 30] Adjust amount of rooms. If rooms needed is 0, zone complete. False, check which rooms are needed.
  (Math|Integer|DecrementInt (Variables|ZoneDetails|GetRoom%20Needed)
    (:%20%20
      (Variables|ZoneDetails|SetDelete%20Current 0)
      (Utilities|Array|Add (Variables|Components|GetDoor%20List) (Variables|Components|GetSelected%20Exit%20Point))
      (if (== (Variables|ZoneDetails|GetRoom%20Needed) 0)
        (CallFunction|GenerationDone)
        (else
          (CallFunction|CheckRooms))))))

(event Custom|Reset%20Zone
  ;[0.3787 0.6401 1 0.6 30] Reset the zone
  (for _array_element (Variables|Components|GetGenerated%20List)
    (Actor|DestroyActor _array_element))
  (Variables|Timer|SetZone%20Build%20Time (+ (Variables|Timer|GetTimer%20Seconds) (Variables|Timer|GetExtra%20Build%20Time)))
  (CallFunction|ResetZoneDetails)
  (Math|Integer|IncrementInt (Variables|ZoneDetails|GetZone%20Reset%20Current)))

(event Custom|Spawn%20Starting%20Room
  (bind _exit_list (Variables|Components|GetExit%20List))
  (bind _outitem (Utilities|Array|Random _exit_list))
  ;[0.3787 0.6401 1 0.6 30] Spawn the starting room
  (Utilities|FlowControl|Delay (Variables|Time|GetTime%20Between%20Rooms))
  (Variables|RoomDetails|SetbTryStartingRoom true)
  (Utilities|IsValid _outitem
    (:Is%20Valid
      (bind _output_get (Variables|Components|SetSelected%20Exit%20Point _outitem))
      (bind _returnvalue (Game|SpawnActorfromClass "/Game/EOTA/Blueprints/Actor/Dungeon/Rooms/Starting/BP_Dungeon_StartHallway.BP_Dungeon_StartHallway_C" (Transformation|GetWorldTransform _output_get) "AlwaysSpawn" "MultiplyWithRoot" 0 0))
      (bind _output_get_2 (Variables|Components|SetLatest%20Room _returnvalue))
      (Utilities|Array|Add (Variables|Components|GetGenerated%20List) _output_get_2)
      (CallFunction|AddOverlapRooms))))

(event Custom|Generation%20Done
  ;[0.3787 0.6401 1 0.6 30] Room generation is complete
  (Utilities|Time|ClearandInvalidateTimerbyHandle (Variables|Timer|GetDungeon%20Timer%20Handle))
  (CallFunction|SpawnExitWalls)
  (CallFunction|SpawnDoorFrames)
  (Development|PrintString "Zone Complete" true true "(R=0.960229,G=1.000000,B=0.255208,A=1.000000)")
  (CallFunction|SpawnNextZone))

(event Custom|Increase%20Challenge%20Room%20Chance
  (bind _ch_room_chance (Variables|Default|GetCH%20Room%20Chance))
  (bind _returnvalue (Utilities|Array|Length _ch_room_chance))
  ;[0.3787 0.6401 1 0.6 30] Increase the challenge room chance
  (if (>= _returnvalue 0)
    (Utilities|Array|RemoveIndex (Variables|Default|GetCH%20Room%20Chance) (- _returnvalue 1))))

(event Custom|Delete%20Room
  (bind _latest_room (Variables|Components|GetLatest%20Room))
  ;[0.3787 0.6401 1 0.6 30] Destroy actor, remove from the overlap list, and generated room list
  (Utilities|Array|Clear (Variables|Components|GetOverlapping%20List))
  (Actor|DestroyActor _latest_room)
  (Utilities|Array|RemoveItem (Variables|Components|GetGenerated%20List) _latest_room))

(event Custom|Check%20Rooms
  ;[0.3787 0.6401 1 0.6 30] Check to make sure all rooms are generated. If the last not, dungeon is valid.
  (if (Utilities|Array|IsEmpty (Variables|Components|GetExit%20List))
    (CallFunction|ResetZone)
    (Development|PrintString "LIST RESET" true true "(R=0.630208,G=0.203505,B=0.203505,A=1.000000)" 4.0)
    (CallFunction|SetupDungeon)
    (elif (not (Variables|RoomDetails|GetbHasStartingRoom))
      (CallFunction|SpawnStartingRoom)
      (elif (not (Variables|RoomDetails|GetbHasChallengeRoom))
        (bind _out_room (CallFunction|GetRandomChallengeRoom))
        (switch int _out_room
          (:0
            (CallFunction|SpawnSwitchChallenge))
          (:1
            (CallFunction|SpawnLightChallenge)))
        (elif (and (== (Variables|ZoneDetails|GetRoom%20Needed) 1) (not (Variables|RoomDetails|GetbHasRelicRoom)))
          (CallFunction|SpawnRelicRoom)
          (else
            (CallFunction|SpawnRandomRoom)))))))

(event Custom|Spawn%20Relic%20Room
  (bind _exit_list (Variables|Components|GetExit%20List))
  (bind _outitem (Utilities|Array|Random _exit_list))
  ;[0.3787 0.6401 1 0.6 30] Spawn Relic Room
  (Utilities|FlowControl|Delay (Variables|Time|GetTime%20Between%20Rooms))
  (Variables|RoomDetails|SetbTryRelicRoom true)
  (Utilities|IsValid _outitem
    (:Is%20Valid
      (bind _output_get (Variables|Components|SetSelected%20Exit%20Point _outitem))
      (bind _returnvalue (Game|SpawnActorfromClass "/Game/EOTA/Blueprints/Actor/Dungeon/Rooms/Special/BP_Dungeon_RelicRoom.BP_Dungeon_RelicRoom_C" (Transformation|GetWorldTransform _output_get) "AlwaysSpawn" "MultiplyWithRoot" 0 0))
      (bind _output_get_2 (Variables|Components|SetRelic%20Room _returnvalue))
      (bind _output_get_3 (Variables|Components|SetLatest%20Room _output_get_2))
      (Utilities|Array|Add (Variables|Components|GetGenerated%20List) _output_get_3)
      (CallFunction|AddOverlapRooms))))

(event Custom|Check%20Relic
  (if (> (Variables|ZoneDetails|GetRelic%20Fail%20Current) (Variables|ZoneDetails|GetRelic%20Limit))
    (CallFunction|ResetZone)
    (Development|PrintString "RELIC RESET" true true "(R=0.630208,G=0.203505,B=0.203505,A=1.000000)" 4.0)
    (CallFunction|SetupDungeon)
    (else
      (CallFunction|SpawnRelicRoom))))

(event Custom|Add%20Overlap%20Rooms
  ;[0.3787 0.6401 1 0.6 30] Add any rooms that overlap with the latest room to the overlapping list
  (for _array_element (Components|GetChildrenComponents (Variables|/Game/EOTA/Blueprints/Actor/Dungeon/BP_Dungeon_MasterRoom.BP_Dungeon_MasterRoom_C|GetOverlap%20Folder (Variables|Components|GetLatest%20Room)) false)
    (bind _asbox_collision (Utilities|Casting|CastToBoxComponent _array_element))
    (Utilities|Array|AppendArray (Variables|Components|GetOverlapping%20List) (Class|PrimitiveComponent|GetOverlappingComponents _asbox_collision)))
  (CallFunction|CheckOverlap))

(event Custom|Spawn%20Light%20Challenge
  (bind _exit_list (Variables|Components|GetExit%20List))
  (bind _outitem (Utilities|Array|Random _exit_list))
  ;[0.3787 0.6401 1 0.6 30] Spawn Light Challenge Room
  (Utilities|FlowControl|Delay (Variables|Time|GetTime%20Between%20Rooms))
  (Variables|RoomDetails|SetbTryChallengeRoom true)
  (Utilities|IsValid _outitem
    (:Is%20Valid
      (bind _output_get (Variables|Components|SetSelected%20Exit%20Point _outitem))
      (bind _returnvalue (Game|SpawnActorfromClass "/Game/EOTA/Blueprints/Actor/Dungeon/Rooms/Challenge/BP_Dungeon_CH_Light.BP_Dungeon_CH_Light_C" (Transformation|GetWorldTransform _output_get) "Undefined" "MultiplyWithRoot" 0 0))
      (bind _output_get_2 (Variables|Components|SetLight%20Room _returnvalue))
      (bind _output_get_3 (Variables|Components|SetLatest%20Room _output_get_2))
      (Utilities|Array|Add (Variables|Components|GetGenerated%20List) _output_get_3)
      (CallFunction|AddOverlapRooms))))

(event Custom|Spawn%20Next%20Zone
  ;[0.6302 0.2035 0.2035 0.5 30] Spawn the next zone from the main dungeon manager
  (Default|SpawnZone (Variables|Components|GetBP%20Dungeon%20Generator%20Main) (Variables|Timer|GetZone%20Build%20Time))
  (Variables|Timer|SetZone%20Build%20Time 0))

(event Custom|Spawn%20Switch%20Challenge
  (bind _exit_list (Variables|Components|GetExit%20List))
  (bind _outitem (Utilities|Array|Random _exit_list))
  ;[0.3787 0.6401 1 0.6 30] Spawn Switch Challenge Room
  (Utilities|FlowControl|Delay (Variables|Time|GetTime%20Between%20Rooms))
  (Variables|RoomDetails|SetbTryChallengeRoom true)
  (Utilities|IsValid _outitem
    (:Is%20Valid
      (bind _output_get (Variables|Components|SetSelected%20Exit%20Point _outitem))
      (bind _returnvalue (Game|SpawnActorfromClass "/Game/EOTA/Blueprints/Actor/Dungeon/Rooms/Challenge/BP_Dungeon_CH_Switch.BP_Dungeon_CH_Switch_C" (Transformation|GetWorldTransform _output_get) "Undefined" "MultiplyWithRoot" 0 0))
      (bind _output_get_2 (Variables|Components|SetLatest%20Room _returnvalue))
      (Utilities|Array|Add (Variables|Components|GetGenerated%20List) _output_get_2)
      (CallFunction|AddOverlapRooms))))

(event Custom|Check%20Overlap
  ;[0.3787 0.6401 1 0.6 30] Check room collision. True, delete the room. False, add that room's exits to list, then continue.
  (if (Utilities|Array|IsNotEmpty (Variables|Components|GetOverlapping%20List))
    (CallFunction|DeleteRoom)
    (Math|Integer|IncrementInt (Variables|ZoneDetails|GetDelete%20Current)
      (:%20%20
        (if (Variables|RoomDetails|GetbTryRelicRoom)
          (Math|Integer|IncrementInt (Variables|ZoneDetails|GetRelic%20Fail%20Current)
            (:%20%20
              (CallFunction|CheckRelic)))
          (else
            (CallFunction|CheckDelete)
            (CallFunction|CheckRooms)))))
    (else
      (bind _output_exit_list (CallFunction|GetAllExits))
      (Utilities|Array|AppendArray (Variables|Components|GetExit%20List) _output_exit_list)
      (Utilities|Array|RemoveItem (Variables|Components|GetExit%20List) (Variables|Components|GetSelected%20Exit%20Point))
      (if (Variables|RoomDetails|GetbTryStartingRoom)
        (Variables|RoomDetails|SetbHasStartingRoom true)
        (Variables|RoomDetails|SetbTryStartingRoom false))
      (if (Variables|RoomDetails|GetbTryChallengeRoom)
        (Variables|RoomDetails|SetbHasChallengeRoom true)
        (Variables|RoomDetails|SetbTryChallengeRoom false))
      (if (Variables|RoomDetails|GetbTryRelicRoom)
        (Variables|RoomDetails|SetbHasRelicRoom true)
        (Variables|RoomDetails|SetbTryRelicRoom false)
        (else
          (Variables|Components|SetRelic%20Room 0)))
      (CallFunction|SetRoom))))

(event Custom|Spawn%20Door%20Frames
  ;[0.3787 0.6401 1 0.6 30] Spawn a door frame at each exit that is connected to a room
  (for _array_element (Variables|Components|GetDoor%20List)
    (Game|SpawnActorfromClass (.OutItem (Utilities|Array|Random (Variables|RoomLists|GetDoor%20Actor%20List))) (Transformation|GetWorldTransform _array_element) "AlwaysSpawn" "MultiplyWithRoot" 0 0)))

(event Custom|Spawn%20Exit%20Walls
  ;[0.3787 0.6401 1 0.6 30] Place exit walls at the exits not connected to any room
  (for _array_element (Variables|Components|GetExit%20List)
    (Game|SpawnActorfromClass "/Game/EOTA/Blueprints/Actor/Dungeon/Walls/BP_Dungeon_Exit_Wall.BP_Dungeon_Exit_Wall_C" (Transformation|GetWorldTransform _array_element) "AlwaysSpawn" "MultiplyWithRoot" 0 0)))

(event Custom|Start%20Dungeon%20Timer
  ;[0.07484 0.2384 0.4635 0.6 30] Start the stopwatch clock to track how long it takes to create
  (bind _returnvalue (Utilities|Time|SetTimerbyEvent (delegate Custom|Dungeon%20Timer%20Tick) 1.0 true))
  (Variables|Timer|SetDungeon%20Timer%20Handle _returnvalue))

(event Custom|Dungeon%20Timer%20Tick
  ;[0.07484 0.2384 0.4635 0.6 30] Start the stopwatch clock to track how long it takes to create
  (Development|PrintText (Utilities|Text|FormatText (Utilities|Text|ToText(Integer) (Variables|Timer|GetTimer%20Seconds))) true true "(R=0.596293,G=1.000000,B=0.496001,A=1.000000)")
  (bind _result (Math|Integer|IncrementInt (Variables|Timer|GetTimer%20Seconds))
    (:%20%20
      (if (>= _result (Variables|Timer|GetBuild%20Time%20Limit))
        (Development|PrintString "OUT OF TIME" true true "(R=1.000000,G=0.286837,B=0.270833,A=1.000000)")
        (Utilities|Time|PauseTimerbyHandle (Variables|Timer|GetDungeon%20Timer%20Handle))
        (Variables|Timer|SetExtra%20Build%20Time (+ (Variables|Timer|GetTimer%20Seconds) (Variables|Timer|GetExtra%20Build%20Time)))
        (CallFunction|ResetZone)
        (Development|PrintString "TIME RESET" true true "(R=0.630208,G=0.203505,B=0.203505,A=1.000000)" 4.0)
        (CallFunction|SetupDungeon)))))

(event Custom|Setup%20Dungeon
  (bind _room_goal (Variables|ZoneDetails|GetRoom%20Goal))
  ;[0.3787 0.6401 1 0.6 30] Set the values for the dungeon before starting the timer
  (CallFunction|StartDungeonTimer)
  (bind _ouput_zone_exit (CallFunction|GetZoneExit))
  (Utilities|Array|Add (Variables|Components|GetExit%20List) _ouput_zone_exit)
  (Variables|ZoneDetails|SetRoom%20Needed _room_goal)
  (Variables|Timer|SetBuild%20Time%20Limit (+ (/ _room_goal 2) 2))
  (CallFunction|SetChallengeRoomChance)
  (CallFunction|SpawnStartingRoom))

(event Custom|Hard%20Reset
  (Game|OpenLevel(byObjectReference) "/Game/EOTA/Maps/MAP_MainDungeon.MAP_MainDungeon"))

(event EventBeginPlay
  (CallFunction|SetupDungeon))

(fn ConstructionScript)

(fn SetHasStartingRoom
  (Variables|RoomDetails|SetbHasStartingRoom true)
  (Variables|RoomDetails|SetbTryStartingRoom false))

(fn SetHasChallengeRoom
  (Variables|RoomDetails|SetbHasChallengeRoom true)
  (Variables|RoomDetails|SetbTryChallengeRoom false))

(fn SetChallengeRoomChance
  (bind _room_goal (Variables|ZoneDetails|GetRoom%20Goal))
  (bind _returnvalue (- _room_goal 2))
  (bind _output_get (LocalVariables|SetTemp%20Room%20Goal _returnvalue))
  (while (> _output_get 0)
    (if (== (LocalVariables|GetTemp%20Room%20Goal) _returnvalue)
      (Utilities|Array|Add (Variables|Default|GetCH%20Room%20Chance) 1)
      (else
        (Utilities|Array|Add (Variables|Default|GetCH%20Room%20Chance) 0)))
    (Math|Integer|DecrementInt (LocalVariables|GetTemp%20Room%20Goal))))

(fn GetAllExits
  (return (Components|GetChildrenComponents (Variables|/Game/EOTA/Blueprints/Actor/Dungeon/BP_Dungeon_MasterRoom.BP_Dungeon_MasterRoom_C|GetExit%20Folder (Variables|Components|GetLatest%20Room)) false)))

(fn GetZoneExit
  (bind _returnvalue (Actor|GetActorOfClass "/Game/EOTA/Blueprints/Dungeon/BP_Dungeon_Manager.BP_Dungeon_Manager_C"))
  (Utilities|IsValid _returnvalue
    (:Is%20Valid
      (bind _output_get (Variables|Components|SetBP%20Dungeon%20Generator%20Main _returnvalue))
      (return (Variables|/Game/EOTA/Blueprints/Dungeon/BP_Dungeon_Manager.BP_Dungeon_Manager_C|GetZone%20Exit _output_get)))
    (:Is%20Not%20Valid
      (Development|PrintString "NOT VALID CAST"))))

(fn PickChallengeRoom
  (return (== (.OutItem (Utilities|Array|Random (Variables|Default|GetCH%20Room%20Chance))) 1)))

(fn ResetZoneDetails
  (Utilities|Time|ClearandInvalidateTimerbyHandle (Variables|Timer|GetDungeon%20Timer%20Handle))
  (Utilities|FlowControl|Sequence
    (:then_0
      (Utilities|Array|Clear (Variables|Components|GetGenerated%20List))
      (Variables|RoomDetails|SetbHasChallengeRoom false)
      (Variables|RoomDetails|SetbTryStartingRoom false)
      (Variables|RoomDetails|SetbTryRelicRoom false))
    (:then_1
      (Utilities|Array|Clear (Variables|Components|GetExit%20List))
      (Variables|RoomDetails|SetbHasStartingRoom false)
      (Variables|RoomDetails|SetbTryChallengeRoom false)
      (Variables|RoomDetails|SetbHasRelicRoom false))
    (:then_2
      (Utilities|Array|Clear (Variables|Components|GetDoor%20List))
      (Variables|ZoneDetails|SetRoom%20Needed (Variables|ZoneDetails|GetRoom%20Goal))
      (Variables|Timer|SetTimer%20Seconds 1)
      (Utilities|Array|Clear (Variables|Default|GetCH%20Room%20Chance))
      (Variables|ZoneDetails|SetRelic%20Fail%20Current 0)
      (Variables|ZoneDetails|SetDelete%20Current 0))))

(fn SpawnRelicAltar
  (params (Enum%20Relic%20Type :type Enum_RelicType%20Enum :default "NewEnumerator6"))
  (bind _out_relic_spawnpoint (Default|GetRelicSpawnpoint (Variables|Components|GetRelic%20Room)))
  (Game|SpawnActorfromClass "/Game/EOTA/Blueprints/Actor/BP_AltarRelic.BP_AltarRelic_C" (Math|Transform|MakeTransform (Transformation|GetWorldLocation _out_relic_spawnpoint) (Transformation|GetWorldRotation _out_relic_spawnpoint) "1.000000,1.000000,1.000000") "Undefined" "MultiplyWithRoot" 0 Enum%20Relic%20Type 0))

(fn SpawnLightEmitter
  (bind _light_room (Variables|Components|GetLight%20Room))
  (Utilities|IsValid _light_room
    (:Is%20Valid
      (bind _out_spawnpoints (Default|GetEmitterSpawnpoints _light_room))
      (Game|SpawnActorfromClass "/Game/EOTA/Blueprints/Actor/BP_LightEmitter.BP_LightEmitter_C" (Math|Transform|MakeTransform (Transformation|GetWorldLocation (.OutItem (Utilities|Array|Random _out_spawnpoints))) (Transformation|GetWorldRotation (.OutItem (Utilities|Array|Random _out_spawnpoints))) "1.000000,1.000000,1.000000") "Undefined" "MultiplyWithRoot" 0 0))))

(fn GetRandomChallengeRoom
  (return (.OutIndex (Utilities|Array|Random (Variables|RoomLists|GetChallenge%20Room%20List)))))