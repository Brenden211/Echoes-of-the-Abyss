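; Dungeon switch challenge that randomly wires levers to wooden doors when play begins.
; It gathers child actor components from scene folders into three lever zones and six door rows.
; First, middle and last passes pair each zone's levers with two rows through BP_Lever, removing only some picked doors and no levers from the lists.
; A separate LeverToggleDoor event toggles a given BP_Door_Wood.
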(event Custom|Set%20Lever%20Lists
  ;[1 0.9459 0 1 30] Set the lever lists to components inside the scene folder
  (bind _out_lever_list (CallFunction|SetLeverList (Variables|Default|GetLever%20Folder%20A)))
  (Variables|Default|SetLever%20ListA _out_lever_list)
  (bind _out_lever_list_2 (CallFunction|SetLeverList (Variables|Default|GetLever%20Folder%20B)))
  (Variables|Default|SetLever%20ListB _out_lever_list_2)
  (bind _out_lever_list_3 (CallFunction|SetLeverList (Variables|Default|GetLever%20Folder%20C)))
  (Variables|Default|SetLever%20ListC _out_lever_list_3))

(event Custom|Set%20Door%20to%20Lever
  ;[0.3787 0.6401 1 1 30] Call set the door to the lever
  (CallFunction|CastSetLevertoDoor (Variables|Default|GetSelected%20Lever) (Variables|Default|GetSelected%20Door)))

(event Custom|Lever%20Toggle%20Door
  (params (In%20Door :type Actor%20Object%20Reference))
  ;[0.3787 0.6401 1 1 30] Call toggle door with the door
  (CallFunction|CastToggleDoor In%20Door))

(event Custom|Select%20Random%20Door%20and%20Lever
  (params (In%20Lever%20List :type Array%20of%20Child%20Actor%20Component%20Object%20References) (In%20Door%20List :type Array%20of%20Child%20Actor%20Component%20Object%20References))
  ;[0.3787 0.6401 1 1 30] Randomly set the door and lever and remove them from their list
  (bind (_out_lever _out_lever_child) (CallFunction|SelectRandomLever In%20Lever%20List))
  (Variables|Default|SetSelected%20Lever _out_lever)
  (Variables|Default|SetSelected%20Lever%20Child _out_lever_child)
  (bind (_out_door _out_door_child) (CallFunction|SelectRandomDoor In%20Door%20List))
  (Variables|Default|SetSelected%20Door _out_door)
  (Variables|Default|SetSelected%20Door%20Child _out_door_child)
  (CallFunction|SetDoortoLever))

(event Custom|Set%20Door%20Lists
  ;[1 0.9459 0 1 30] Set the door lists to components inside the scene folder
  (bind _out_door_list (CallFunction|SetDoorList (Variables|Default|GetDoor%20Folder%20A)))
  (Variables|Default|SetDoorListA _out_door_list)
  (bind _out_door_list_2 (CallFunction|SetDoorList (Variables|Default|GetDoor%20Folder%20B)))
  (Variables|Default|SetDoorListB _out_door_list_2)
  (bind _out_door_list_3 (CallFunction|SetDoorList (Variables|Default|GetDoor%20Folder%20C)))
  (Variables|Default|SetDoorListC _out_door_list_3)
  (bind _out_door_list_4 (CallFunction|SetDoorList (Variables|Default|GetDoor%20Folder%20D)))
  (Variables|Default|SetDoorListD _out_door_list_4)
  (bind _out_door_list_5 (CallFunction|SetDoorList (Variables|Default|GetDoor%20Folder%20E)))
  (Variables|Default|SetDoorListE _out_door_list_5)
  (bind _out_door_list_6 (CallFunction|SetDoorList (Variables|Default|GetDoor%20Folder%20F)))
  (Variables|Default|SetDoorListF _out_door_list_6))

(event Custom|Door%20Assign%20First
  (bind _doorlistb (Variables|Default|GetDoorListB))
  (bind _doorlista (Variables|Default|GetDoorListA))
  (bind _doorlistb_2 (Variables|Default|GetDoorListB))
  ;[0.3787 0.6401 1 1 30] Set the starting section
  ;;[0.3787 0.6401 1] Assign 1 lever from zone A to 1 door in row A
  (CallFunction|SelectRandomDoorandLever (Variables|Default|GetLever%20ListA) _doorlista)
  (Utilities|Array|RemoveItem _doorlista (Variables|Default|GetSelected%20Door%20Child))
  ;;[0.3787 0.6401 1] Assign 2 levers from zone A to 2 different doors in the row B
  (CallFunction|SelectRandomDoorandLever (Variables|Default|GetLever%20ListA) _doorlistb_2)
  (Utilities|Array|RemoveItem _doorlistb_2 (Variables|Default|GetSelected%20Door%20Child))
  (CallFunction|SelectRandomDoorandLever (Variables|Default|GetLever%20ListA) _doorlistb)
  (Utilities|Array|RemoveItem _doorlistb (Variables|Default|GetSelected%20Door%20Child)))

(event Custom|Door%20Assign%20Last
  (bind _doorlistf (Variables|Default|GetDoorListF))
  (bind _doorlistf_2 (Variables|Default|GetDoorListF))
  (for _index (range 0 3)
    (CallFunction|SelectRandomDoorandLever (Variables|Default|GetLever%20ListC) (Variables|Default|GetDoorListE)))
  (CallFunction|SelectRandomDoorandLever (Variables|Default|GetLever%20ListC) _doorlistf_2)
  (Utilities|Array|RemoveItem _doorlistf_2 (Variables|Default|GetSelected%20Door%20Child))
  (CallFunction|SelectRandomDoorandLever (Variables|Default|GetLever%20ListC) _doorlistf)
  (Utilities|Array|RemoveItem _doorlistf (Variables|Default|GetSelected%20Door%20Child)))

(event Custom|Door%20Assign%20Middle
  (bind _doorlistd (Variables|Default|GetDoorListD))
  (bind _doorlistd_2 (Variables|Default|GetDoorListD))
  (for _index (range 0 6)
    (CallFunction|SelectRandomDoorandLever (Variables|Default|GetLever%20ListB) (Variables|Default|GetDoorListC)))
  (CallFunction|SelectRandomDoorandLever (Variables|Default|GetLever%20ListB) _doorlistd)
  (Utilities|Array|RemoveItem _doorlistd (Variables|Default|GetSelected%20Door%20Child))
  (CallFunction|SelectRandomDoorandLever (Variables|Default|GetLever%20ListB) _doorlistd_2)
  (Utilities|Array|RemoveItem _doorlistd_2 (Variables|Default|GetSelected%20Door%20Child)))

(event EventBeginPlay
  (|CallParentFunction)
  (CallFunction|SetLeverLists)
  (CallFunction|SetDoorLists)
  (CallFunction|DoorAssignFirst)
  (CallFunction|DoorAssignMiddle)
  (CallFunction|DoorAssignLast))

(fn ConstructionScript
  (|CallParentFunction))

(fn SetDoorList
  (params (In%20Door%20Folder :type Scene%20Component%20Object%20Reference))
  (for _array_element (Components|GetChildrenComponents In%20Door%20Folder false)
    (bind _aschild_actor_component (Utilities|Casting|CastToChildActorComponent _array_element))
    (Utilities|Array|Add (LocalVariables|GetDoorList) _aschild_actor_component))
  (return (LocalVariables|GetDoorList)))

(fn CastToggleDoor
  (params (In%20Door :type Actor%20Object%20Reference))
  (bind _asbp_doorway_wood (Utilities|Casting|CastToBP_Door_Wood In%20Door))
  (Default|ToggleDoor _asbp_doorway_wood))

(fn SelectRandomDoor
  (params (In%20Door%20List :type Array%20of%20Child%20Actor%20Component%20Object%20References))
  (LocalVariables|SetDoorList In%20Door%20List)
  (if (> (Utilities|Array|Length (LocalVariables|GetDoorList)) 0)
    (return (Variables|/Script/Engine.ChildActorComponent|GetChildActor (.OutItem (Utilities|Array|Random (LocalVariables|GetDoorList)))) (.OutItem (Utilities|Array|Random (LocalVariables|GetDoorList))))))

(fn SetLeverList
  (params (In%20Lever%20Folder :type Scene%20Component%20Object%20Reference))
  (for _array_element (Components|GetChildrenComponents In%20Lever%20Folder false)
    (bind _aschild_actor_component (Utilities|Casting|CastToChildActorComponent _array_element))
    (Utilities|Array|Add (LocalVariables|GetLever%20List) _aschild_actor_component))
  (return (LocalVariables|GetLever%20List)))

(fn CastSetLevertoDoor
  (params (In%20Lever :type Actor%20Object%20Reference) (In%20Door :type Actor%20Object%20Reference))
  (bind _asbp_lever (Utilities|Casting|CastToBP_Lever In%20Lever))
  (Default|SetDoortoLever _asbp_lever In%20Door))

(fn SelectRandomLever
  (params (In%20Lever%20List :type Array%20of%20Child%20Actor%20Component%20Object%20References))
  (LocalVariables|SetLeverList In%20Lever%20List)
  (if (> (Utilities|Array|Length (LocalVariables|GetLeverList)) 0)
    (return (Variables|/Script/Engine.ChildActorComponent|GetChildActor (.OutItem (Utilities|Array|Random (LocalVariables|GetLeverList)))) (.OutItem (Utilities|Array|Random (LocalVariables|GetLeverList))))))