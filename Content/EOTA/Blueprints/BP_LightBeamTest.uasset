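; BP_LightBeamTest is a test actor that fires a particle light beam forward from its cube on BeginPlay.
; It attaches the beam emitter, then runs a visibility line trace along the cube's forward vector.
; On a hit, it sets beam endpoints, combining the hit component's X with its own Y/Z, then adding its location again.
; On a miss, it prints a message and draws a debug line.
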(event Custom|Activate%20Beam
  (Utilities|FlowControl|Sequence
    (:then_0
      (bind _returnvalue (Effects|SpawnEmitterAttached "/Game/EOTA/Niagara/CP_LightBeam.CP_LightBeam" (Variables|Default|GetCube) "None"))
      (Variables|Default|SetLightParticle _returnvalue)
      (bind _outhit (Collision|LineTraceByChannel (Variables|Default|GetSelf%20Location) (+ (Variables|Default|GetSelf%20Location) (Variables|Default|GetEnd%20Location)) "TraceTypeQuery1" false 0 "None" true "(R=1.000000,G=0.000000,B=0.000000,A=1.000000)" "(R=0.000000,G=1.000000,B=0.000000,A=1.000000)" 1e+01))
      (Utilities|IsValid (.hitcomponent _outhit)
        (:Is%20Valid
          (Variables|Default|SetEnd%20Hit%20Location (+ (* (Transformation|GetWorldLocation (.hitcomponent _outhit)) "1.000000,0.000000,0.000000") (* (Variables|Default|GetSelf%20Location) "0.000000,1.000000,1.000000")))
          (Variables|Default|SetIsHit true))
        (:Is%20Not%20Valid
          (Development|PrintString "NO HIT")
          (Rendering|Debug|DrawDebugLine (Variables|Default|GetSelf%20Location) (+ (Variables|Default|GetSelf%20Location) (Variables|Default|GetEnd%20Location)) "(R=0.900354,G=0.270759,B=1.000000,A=1.000000)" 5.0 3.0))))
    (:then_1
      (if (Variables|Default|GetIsHit)
        (Class|ParticleSystemComponent|SetBeamSourcePoint (Variables|Default|GetLightParticle) 0 (Variables|Default|GetSelf%20Location))
        (Class|ParticleSystemComponent|SetBeamEndPoint (Variables|Default|GetLightParticle) 0 (+ (Variables|Default|GetSelf%20Location) (Variables|Default|GetEnd%20Hit%20Location)))))))

(event EventBeginPlay
  (bind _cube (Variables|Default|GetCube))
  (Variables|Default|SetSelf%20Location (Transformation|GetWorldLocation _cube))
  (Variables|Default|SetEnd%20Location (* (Math|Vector|GetForwardVector _cube) 2e+03))
  (CallFunction|ActivateBeam))

(fn ConstructionScript)